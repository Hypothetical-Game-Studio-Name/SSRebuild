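; CameraBP is a shared camera actor that follows the midpoint of two characters.
; On BeginPlay it caches all BaseCharacter actors, then every Tick averages the positions of the first two.
; It offsets that point along X by XMin and raises it by ZMin, clamping each character's height contribution to a minimum, while holding a fixed rotation.
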(event `self.ReceiveBeginPlay`
  (bind _outactors (`GameplayStatics.GetAllActorsOfClass` "/Game/Blueprints/CharacterStuff/BaseCharacter.BaseCharacter_C"))
  (set `self.Character Array` _outactors))

(event `self.ReceiveTick`
  (params (DeltaSeconds :type "Float (single-precision)"))
  (bind _zmin (`self.ZMin`))
  (bind _zmin_2 (`self.ZMin`))
  (bind (_returnvalue_x _returnvalue_y _returnvalue_z) (`KismetMathLibrary.BreakVector` (`self.K2_GetActorLocation` (`|GetArrayItem` (`self.Character Array`) 1))))
  (bind (_returnvalue_x_2 _returnvalue_y_2 _returnvalue_z_2) (`KismetMathLibrary.BreakVector` (`self.K2_GetActorLocation` (`|GetArrayItem` (`self.Character Array`)))))
  (`self.K2_SetActorLocationAndRotation` (/ (+ (`KismetMathLibrary.MakeVector` (- _returnvalue_x_2 (`self.XMin`)) _returnvalue_y_2 (`KismetMathLibrary.FClamp` (+ _returnvalue_z_2 _zmin) _zmin 100000.0)) (`KismetMathLibrary.MakeVector` (- _returnvalue_x (`self.XMin`)) _returnvalue_y (`KismetMathLibrary.FClamp` (+ _returnvalue_z _zmin_2) _zmin_2 100000.0))) 2.0) (struct :`Pitch` -80.0)))

(fn `UserConstructionScript`)