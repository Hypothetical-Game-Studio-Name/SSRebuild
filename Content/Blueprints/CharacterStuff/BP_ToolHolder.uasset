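; BP_ToolHolder is a holder that passes tools to and from a BaseCharacter through PassMessage and displays the held tool.
; When Holding, it gives the character its tool, clears Holding and resets to ElectricGun.
; Otherwise it copies the character's tool, but the nodes setting Holding and the character's tool to Hammer are unconnected.
; ChangeTool swaps the Cube1 mesh to match, with Electric Gun showing no mesh.
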(event `/Game/Interfaces/InteractInterface.PassMessage`
  (params (SourceRef :type "Actor Object Reference"))
  (if (`self.Holding?`)
    (bind _asbase_character (cast `/Game/Blueprints/CharacterStuff/BaseCharacter` SourceRef))
    (set `/Game/Blueprints/CharacterStuff/BaseCharacter.CurrentTool` (`self.CurrentHeldTool`) _asbase_character)
    (set `self.Holding?` false)
    (bind _output_get (set `self.CurrentHeldTool` "NewEnumerator2"))
    (`self.ChangeTool` _output_get)
    (else
      (bind _asbase_character_2 (cast `/Game/Blueprints/CharacterStuff/BaseCharacter` SourceRef))
      (bind _output_get_2 (set `self.CurrentHeldTool` (`/Game/Blueprints/CharacterStuff/BaseCharacter.CurrentTool` _asbase_character_2)))
      (`self.ChangeTool` _output_get_2))))

(event `ChangeTool`
  (params (ChangeToo :type "/Game/Blueprints/Tools/ToolEnum Enum" :default "NewEnumerator0"))
  (bind _cube1 (`self.Cube1`))
  (switch `/Game/Blueprints/Tools/ToolEnum` ChangeToo
    (:`NewEnumerator0`
      (`StaticMeshComponent.SetStaticMesh` _cube1 "/Game/Meshes/Hammer.Hammer"))
    (:`NewEnumerator1`
      (`StaticMeshComponent.SetStaticMesh` _cube1 "/Game/Meshes/FEMesh.FEMesh"))
    (:`NewEnumerator2`
      (`StaticMeshComponent.SetStaticMesh` _cube1 null))))

(fn `UserConstructionScript`)