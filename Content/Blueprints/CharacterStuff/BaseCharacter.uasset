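; Base player character that handles movement, swept timeline dash, timed emote flags, hazard damage and death, and randomly picks one of two skins on construction.
; Sphere traces drive slapping and interacting, limited to level-select actors in menus; held barrels are placed by trace.
; The held tool is a child actor defaulting to the hammer: pickup swaps its class, while throw/drop spawns an outlined copy and restores the hammer, passing state via GetToolInfoMessage.
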(event `HahaAnim`
  ;[1 1 1] Emotes
  (set `self.Haha` true)
  (`KismetSystemLibrary.K2_SetTimerDelegate` (delegate `ResetHaha`) 1.4))

(event `/Game/Blueprints/Interfaces/InteractEvent.Is Slapped`
  (params (CharacterWhoSlapped :type "/Game/Blueprints/CharacterStuff/BaseCharacter Object Reference"))
  (set `self.IsSlapStunned` true)
  (`KismetSystemLibrary.Delay` 1.5)
  (set `self.IsSlapStunned` false))

(event `ResetHaha`
  ;[1 1 1] Emotes
  (set `self.Haha` false))

(event `WinLevel`
  ;[1 1 1] Win and Lose
  (`/Engine/EditorBlueprintResources/StandardMacros.DoOnce` false
    (:`Completed`
      (set `self.WeWon` true)
      (`KismetSystemLibrary.K2_SetTimerDelegate` (delegate `Reset`) 1.9))))

(event `EmoteNiceone`
  ;[1 1 1] Emotes
  (set `self.Niceone` true)
  (`KismetSystemLibrary.K2_SetTimerDelegate` (delegate `ResetNice`) 1.17))

(event `Reset`
  ;[1 1 1] Win and Lose
  (set `self.WeWon` false))

(event `ResetNice`
  ;[1 1 1] Emotes
  (set `self.Niceone` false))

(event `Loselevel`
  ;[1 1 1] Win and Lose
  (`/Engine/EditorBlueprintResources/StandardMacros.DoOnce` false
    (:`Completed`
      (set `self.We Lose` true)
      (`KismetSystemLibrary.K2_SetTimerDelegate` (delegate `ResetLose`) 1.5))))

(event `EmoteWow`
  ;[1 1 1] Emotes
  (set `self.Wow` true)
  (`KismetSystemLibrary.K2_SetTimerDelegate` (delegate `WowReset`) 1.5))

(event `ResetLose`
  ;[1 1 1] Win and Lose
  (set `self.We Lose` false))

(event `WowReset`
  ;[1 1 1] Emotes
  (set `self.Wow` false))

(event `self.ReceiveBeginPlay`
  (bind _tool_ref (message `/Game/Blueprints/Interfaces/ToolInterafce.Get tool Info` (`ChildActorComponent.ChildActor` (`self.EquippedTool`))))
  (`/Game/Blueprints/Tools/BP_BaseTool.Check if hammer tool is being used by player` _tool_ref)
  ;[1 1 1] Sound
  (`|ExecutionSequence`
    (:`then_0`
      (`PlayerController.SetAudioListenerAttenuationOverride` (`GameplayStatics.GetPlayerController` 0) (`self.Mesh`) (0.0 0.0 0.0)))
    (:`then_1`
      (set `self.original location` (`self.K2_GetActorLocation`))
      (set `self.original rotation` (`self.K2_GetActorRotation`))
      (`KismetSystemLibrary.Delay` 0.2)
      (bind _outactors (`GameplayStatics.GetAllActorsOfClass` "/Game/Blueprints/HazardAssets/CoreHazardClass.CoreHazardClass_C"))
      (set `self.Ignoring Hazards For tool Pickup` _outactors)
      (if (== (`self.GetController`) (`GameplayStatics.GetPlayerControllerFromID` 0))
        _))))

(event `Happy`
  ;[1 1 1] Emotes
  (set `self.HappyEmotes` true)
  (`KismetSystemLibrary.K2_SetTimerDelegate` (delegate `ResetHappy`) 1.5))

(event `SlapEvent`
  (bind _cast_arrow_target (`self.Cast Arrow Target`))
  (bind _returnvalue (`SceneComponent.K2_GetComponentLocation` _cast_arrow_target))
  ;[1 1 1] Slap Event, trace by sphere collision, returns all objects and "Slaps" them.
  (if (`self.InMenu`)
    (bind _outhits (`KismetSystemLibrary.SphereTraceMulti` _returnvalue _returnvalue 100.0 "TraceTypeQuery1"))
    (for _array_element _outhits
      (bind (_bblockinghit _binitialoverlap _time _distance _location _impactpoint _normal _impactnormal _physmat _hitactor) (`GameplayStatics.BreakHitResult` _array_element))
      (if (== (`GameplayStatics.GetObjectClass` _hitactor) "/Game/Blueprints/UI/LevelSelectBP.LevelSelectBP_C")
        (message `/Game/Blueprints/Interfaces/InteractEvent.Is Slapped` _hitactor self)))
    (else
      (bind _outhits_2 (`KismetSystemLibrary.SphereTraceMulti` _returnvalue (+ _returnvalue (* (`KismetMathLibrary.GetForwardVector` (`SceneComponent.K2_GetComponentRotation` _cast_arrow_target)) 300.0)) 50.0 "TraceTypeQuery1"))
      (for _array_element_2 _outhits_2
        (message `/Game/Blueprints/Interfaces/InteractEvent.Is Slapped` (`.HitActor` (`GameplayStatics.BreakHitResult` _array_element_2)) self)))))

(event `ResetHappy`
  ;[1 1 1] Emotes
  (set `self.HappyEmotes` false))

(event `Taking Hazard Effect`
  (params (`Hazard type` :type "/Game/Blueprints/HazardAssets/NatureOfHazard Enum" :default "NewEnumerator0"))
  ;[1 1 1] When the player takes damage from a hazard, these events are fired
  (`ActorComponent.Activate` (`self.Hazard Effect`) false)
  (switch `/Game/Blueprints/HazardAssets/NatureOfHazard` `Hazard type`
    (:`NewEnumerator0`
      (set `self.Onfire` true)
      (set `self.Player Health Before taking damage` (`self.Player Character Health`))
      (bind (_direction _fire_damage_update) (`Timeline|Apply Fire Damage Over time` :!via `PlayFromStart`)
        (:`Update`
          (if (`self.OilSlicked`)
            (set `self.Player Character Health` 0.0)
            (else
              (set `self.Player Character Health` (- (`self.Player Health Before taking damage`) _fire_damage_update))
              (set `self.Onfire` false))))
        (:`Finished`
          (`ActorComponent.Deactivate` (`self.Hazard Effect`)))))))

(event `X-AxisPassEvent`
  (params (Axis :type "Float (double-precision)"))
  ;[1 1 1] Movement
  (if (`self.InMenu`) :!label _label
    _
    (elif (not (`self.Death`))
      (`PawnMovementComponent.AddInputVector` (`self.CharacterMovement`) (`KismetMathLibrary.MakeVector` Axis (stale `Y-AxisPassEvent` Axis)) false))))

(event `Hazard Death Event`
  (params (`Hazard Type` :type "/Game/Blueprints/HazardAssets/NatureOfHazard Enum" :default "NewEnumerator0"))
  ;[1 1 1] When the hazard kills the player, this is the event that the hazard triggers.
  (set `self.Death` true)
  (`self.DisableInput` (`self.ControllerRef`))
  (`KismetSystemLibrary.Delay` 1.5)
  (`/Game/Blueprints/Function_Libraries/NatFunctionLibrary.Player Character Death By Hazard` `Hazard Type` self)
  (set `self.Death` false)
  (`self.EnableInput` (`self.ControllerRef`)))

(event `Y-AxisPassEvent`
  (params (Axis :type "Float (double-precision)"))
  ;[1 1 1] Movement
  (goto _label))

(event `InteractPassEvent`
  (bind _cast_arrow_target (`self.Cast Arrow Target`))
  (bind _returnvalue (`SceneComponent.K2_GetComponentLocation` _cast_arrow_target))
  ;[1 1 1] When the player interacts with something this fires
  (set `self.ObjectInteractedWith` false)
  (if (`self.Holding A Barrel?`)
    (`self.Place Down Barrel`)
    (elif (`self.InMenu`)
      (bind _outhits (`KismetSystemLibrary.SphereTraceMulti` _returnvalue _returnvalue 100.0 "TraceTypeQuery1"))
      (for _array_element _outhits
        (bind (_bblockinghit _binitialoverlap _time _distance _location _impactpoint _normal _impactnormal _physmat _hitactor) (`GameplayStatics.BreakHitResult` _array_element))
        (if (== (`GameplayStatics.GetObjectClass` _hitactor) "/Game/Blueprints/UI/LevelSelectBP.LevelSelectBP_C")
          (message `/Game/Blueprints/Interfaces/InteractEvent.Is interacted with` _hitactor self)))
      (else
        (set `self.InteractAnim` true)
        (bind _outhit (`KismetSystemLibrary.SphereTraceSingle` _returnvalue (+ _returnvalue (* (`KismetMathLibrary.GetForwardVector` (`SceneComponent.K2_GetComponentRotation` _cast_arrow_target)) 300.0)) 40.0 "TraceTypeQuery1"))
        (bind (_bblockinghit_2 _binitialoverlap_2 _time_2 _distance_2 _location_2 _impactpoint_2 _normal_2 _impactnormal_2 _physmat_2 _hitactor_2) (`GameplayStatics.BreakHitResult` _outhit))
        (if (`KismetArrayLibrary.Array_Contains` (`self.InteractableObjects`) (`GameplayStatics.GetObjectClass` _hitactor_2))
          (set `self.ObjectInteractedWith` true)
          (message `/Game/Blueprints/Interfaces/InteractEvent.Is interacted with` _hitactor_2 self)
          (`KismetSystemLibrary.Delay` 1.0)
          (set `self.InteractAnim` false))))))

(event `Dash Event Pass`
  (bind _charactermovement (`self.CharacterMovement`))
  (bind _cast_arrow_target (`self.Cast Arrow Target`))
  ;[1 1 1] New Dash, Sweps over 0.3
  (if (`self.Can Sprint?`)
    (`/Engine/EditorBlueprintResources/StandardMacros.DoOnce` false :!label _label_2
      (:`Completed`
        (set `CharacterMovementComponent.GravityScale` 0.0 _charactermovement)
        (set `self.PreDashLocation` (`SceneComponent.K2_GetComponentLocation` _cast_arrow_target))
        (set `self.Post Dash Location` (+ (`self.PreDashLocation`) (* (`KismetMathLibrary.GetForwardVector` (`SceneComponent.K2_GetComponentRotation` _cast_arrow_target)) 400.0)))
        (bind (_direction _dashalpha) (`Timeline|DashTimeLine` :!via `PlayFromStart`)
          (:`Update`
            (`self.K2_SetActorLocation` (`KismetMathLibrary.VLerp` (`self.PreDashLocation`) (`self.Post Dash Location`) _dashalpha) true))
          (:`Finished`
            (set `CharacterMovementComponent.GravityScale` 1.0 _charactermovement)
            (goto _label_2 :!via `Reset`)))))))

(event `UseToolEvent`
  ;[1 1 1] This is triggered when the tool being held is used
  (`self.F_UseToolFunction`))

(event `StopUsingToolEvent`
  ;[1 1 1] This is triggered when the tool being held is used
  (bind _tool_ref (message `/Game/Blueprints/Interfaces/ToolInterafce.Get tool Info` (`ChildActorComponent.ChildActor` (`self.EquippedTool`))))
  (`/Engine/EditorBlueprintResources/StandardMacros.IsValid` _tool_ref
    (:`Is Valid`
      (`/Game/Blueprints/Tools/BP_BaseTool.ToolStoppedBeingUsed` _tool_ref))))

(event `Pick Up tool`
  (bind _capsulecomponent (`self.CapsuleComponent`))
  (bind (_returnvalue_x _returnvalue_y _returnvalue_z) (`KismetMathLibrary.BreakVector` (`SceneComponent.K2_GetComponentLocation` _capsulecomponent)))
  (bind _returnvalue (`KismetMathLibrary.MakeVector` _returnvalue_x _returnvalue_y (- _returnvalue_z 20.0)))
  ;[1 1 1] Fires a trace to see if any tools that are lying around can be picked up
  (bind _tool_ref (message `/Game/Blueprints/Interfaces/ToolInterafce.Get tool Info` (`ChildActorComponent.ChildActor` (`self.EquippedTool`))))
  (if (`|EnumEquality` (`/Game/Blueprints/Tools/BP_BaseTool.What tool is this?` _tool_ref) "NewEnumerator0")
    (bind (_outhit _returnvalue_2) (`KismetSystemLibrary.SphereTraceSingleForObjects` _returnvalue (+ _returnvalue (* (`SceneComponent.GetForwardVector` _capsulecomponent) 150.0)) (* (`CapsuleComponent.CapsuleRadius` _capsulecomponent) 2.0) (`self.Tool Pick up Search`)))
    (if _returnvalue_2
      (bind _tool_ref_2 (message `/Game/Blueprints/Interfaces/ToolInterafce.Get tool Info` (`.HitActor` (`GameplayStatics.BreakHitResult` _outhit))))
      (`/Engine/EditorBlueprintResources/StandardMacros.IsValid` _tool_ref_2
        (:`Is Valid`
          (if (`/Game/Blueprints/Tools/BP_BaseTool.Can Be picked up?` _tool_ref_2)
            (`/Game/Blueprints/Tools/BP_BaseTool.Set tool passover Information` _tool_ref_2)
            (`ChildActorComponent.SetChildActorClass` (`self.EquippedTool`) (`GameplayStatics.GetObjectClass` _tool_ref_2))
            (bind _tool_ref_3 (message `/Game/Blueprints/Interfaces/ToolInterafce.Get tool Info` (`ChildActorComponent.ChildActor` (`self.EquippedTool`))))
            (`/Game/Blueprints/Tools/BP_BaseTool.Set Tool Variables from passover` _tool_ref_3 (`/Game/Blueprints/Tools/BP_BaseTool.Tool Information To Pass Over` _tool_ref_2))
            (`self.K2_DestroyActor` _tool_ref_2)))))
    (else
      (set `self.HoldingChargeTool` true))))

(event `Key|P`
  (params (Key :type "Key Structure"))
  ;[1 1 1] Testing
  (:`Pressed`
    (`self.Hazard Death Event` "NewEnumerator0")))

(event `Throw own tool`
  (bind _childactor (`ChildActorComponent.ChildActor` (`self.EquippedTool`)))
  (bind (_returnvalue_location _returnvalue_rotation _returnvalue_scale) (`KismetMathLibrary.BreakTransform` (`self.GetTransform` _childactor)))
  ;[1 1 1] When the player throws their tool, this quickly creates a copy of that tool in front of the orginal,
  ; which is NOT apart of the character's child actor. That tool is then told to be thrown,
  ;  while the orginal child actor is deleted. This proccess is so quick, that it is imperceptible to the naked eye.
  (set `self.Throwing / Dropping Strength` 1000.0)
  (bind _tool_ref (message `/Game/Blueprints/Interfaces/ToolInterafce.Get tool Info` (`ChildActorComponent.ChildActor` (`self.EquippedTool`)) :!label _label_3))
  (if (not (`|EnumEquality` (`/Game/Blueprints/Tools/BP_BaseTool.What tool is this?` _tool_ref) "NewEnumerator0"))
    (`/Game/Blueprints/Tools/BP_BaseTool.Set tool passover Information` _tool_ref)
    (bind _returnvalue (`|SpawnActorFromClass` (`ChildActorComponent.ChildActorClass` (`self.EquippedTool`)) (`KismetMathLibrary.MakeTransform` (+ (`self.K2_GetActorLocation` _childactor) (* (`self.GetActorForwardVector` _childactor) 10.0)) _returnvalue_rotation _returnvalue_scale) "Undefined" "OverrideRootScale" null null))
    (bind _tool_ref_2 (message `/Game/Blueprints/Interfaces/ToolInterafce.Get tool Info` _returnvalue))
    (`/Engine/EditorBlueprintResources/StandardMacros.IsValid` _tool_ref_2
      (:`Is Valid`
        (`/Game/Blueprints/Tools/BP_BaseTool.Set Tool Variables from passover` _tool_ref_2 (`/Game/Blueprints/Tools/BP_BaseTool.Tool Information To Pass Over` _tool_ref))
        (`self.Apply Outline to Thrown Tool` _tool_ref_2)
        (`/Game/Blueprints/Tools/BP_BaseTool.Tool is thrown` _tool_ref_2 (`self.Throwing / Dropping Strength`))
        (`ChildActorComponent.SetChildActorClass` (`self.EquippedTool`) "/Game/Blueprints/Tools/BP_HammerTool.BP_HammerTool_C")))))

(event `Drop Own Tool`
  ;[1 1 1] When the player throws their tool, this quickly creates a copy of that tool in front of the orginal,
  ; which is NOT apart of the character's child actor. That tool is then told to be thrown,
  ;  while the orginal child actor is deleted. This proccess is so quick, that it is imperceptible to the naked eye.
  (set `self.HoldingChargeTool` false)
  (set `self.Throwing / Dropping Strength` 10.0)
  (goto _label_3))

(fn `Apply Outline to Thrown Tool`
  (params (`Tool to apply outline` :type "/Game/Blueprints/Tools/BP_BaseTool Object Reference"))
  (bind _toolmesh (`/Game/Blueprints/Tools/BP_BaseTool.ToolMesh` `Tool to apply outline`))
  (`/Engine/EditorBlueprintResources/StandardMacros.IsValid` `Tool to apply outline`
    (:`Is Valid`
      (bind _returnvalue (`AddComponent|NODE_AddStaticMeshComponent-0` :`self` `Tool to apply outline` :`bManualAttachment` true))
      (`PrimitiveComponent.SetCollisionEnabled` _returnvalue "NoCollision")
      (`StaticMeshComponent.SetStaticMesh` _returnvalue (`StaticMeshComponent.StaticMesh` _toolmesh))
      (`SceneComponent.K2_AttachToComponent` _returnvalue _toolmesh "None" "SnapToTarget" "SnapToTarget" "SnapToTarget" true)
      (`PrimitiveComponent.SetMaterial` _returnvalue 0 "/Game/Blueprints/Tools/Outline_Inst.Outline_Inst"))))

(fn `F_UseToolFunction`
  (locals (HazardToEffect :type "/Game/Blueprints/HazardAssets/CoreHazardClass Object Reference"))
  (bind _tool_ref (message `/Game/Blueprints/Interfaces/ToolInterafce.Get tool Info` (`ChildActorComponent.ChildActor` (`self.EquippedTool`))))
  (`/Engine/EditorBlueprintResources/StandardMacros.IsValid` _tool_ref
    (:`Is Valid`
      (`/Game/Blueprints/Tools/BP_BaseTool.ToolIsUsed` _tool_ref null))))

(fn `Place Down Barrel`
  (bind _held_barrel (`self.Held Barrel`))
  (bind _cast_arrow_target (`self.Cast Arrow Target`))
  (bind _held_barrel_2 (`self.Held Barrel`))
  (bind _returnvalue (`SceneComponent.K2_GetComponentLocation` _cast_arrow_target))
  (bind _returnvalue_2 (`self.K2_GetActorLocation` _held_barrel))
  (bind (_outhit _returnvalue_3) (`KismetSystemLibrary.LineTraceSingle` _returnvalue (+ _returnvalue (* (`KismetMathLibrary.GetForwardVector` (`SceneComponent.K2_GetComponentRotation` _cast_arrow_target)) 300.0)) "TraceTypeQuery1" false (`|MakeArray` (`self.Held Barrel`) :!type "Actor Object Reference")))
  (if (not _returnvalue_3)
    (bind _outhit_2 (`KismetSystemLibrary.BoxTraceSingleForObjects` _returnvalue_2 (+ _returnvalue_2 (* (`KismetMathLibrary.Vector_Down`) 300.0)) (32.0 32.0 65.0) (`self.K2_GetActorRotation` _held_barrel) (`|MakeArray` "ObjectTypeQuery1" :!type "EObjectTypeQuery Enum") false (`|MakeArray` _held_barrel :!type "Actor Object Reference")))
    (set `self.Holding A Barrel?` false)
    (`self.K2_DetachFromActor` _held_barrel_2 "KeepWorld" "KeepWorld" "KeepWorld")
    (`/Game/Blueprints/HazardAssets/BarrelsandBoxes/Barrel.Is placed Down` _held_barrel_2 (`.Location` (`GameplayStatics.BreakHitResult` _outhit_2)) self)))

(fn `Player Character Refrence Getter`
  (returns (`Player Character Refrence` :type "/Game/Blueprints/CharacterStuff/BaseCharacter Object Reference"))
  (return self))

(fn `UserConstructionScript`
  (bind _mesh (`self.Mesh`))
  (switch `int` (`KismetMathLibrary.RandomIntegerInRange` 0 1)
    (:`0`
      (`SkinnedMeshComponent.SetSkinnedAssetAndUpdate` _mesh "/Game/Animation/BrickhouseCharacter/Brickhouse_Hammer.Brickhouse_Hammer" true)
      (`SkeletalMeshComponent.SetAnimInstanceClass` _mesh "/Game/Animation/BrickhouseCharacter/BrickAnimBlueprint.BrickAnimBlueprint_C"))
    (:`1`
      (`SkinnedMeshComponent.SetSkinnedAssetAndUpdate` _mesh "/Game/Animation/PhillipNewCharacter/Phillip_Interaction__1_.Phillip_Interaction__1_" true)
      (`SkeletalMeshComponent.SetAnimInstanceClass` _mesh "/Game/Animation/PhillipNewCharacter/PhillipBP1.PhillipBP1_C"))))