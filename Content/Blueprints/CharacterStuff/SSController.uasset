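; Player controller that turns player input into character actions: movement, emotes, interaction, tool use, dash, slap, throw, pickup/drop and pausing.
; Most inputs forward to events on a cached CharacterRef after validity checks, while pause opens the menu on a supplied master UI widget.
; Throw and pickup/drop instead fetch the character from the controlled pawn by message, with the equipped tool's type choosing pickup or drop.
; Dash is rate-limited by a DoOnce reset after a cooldown delay.
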(event `InputAction|NiceOneEmote`
  (params (Key :type "Key Structure"))
  (bind _characterref (`self.CharacterRef`))
  ;[1 1 1] Emotes
  (:`Pressed`
    (`/Engine/EditorBlueprintResources/StandardMacros.IsValid` _characterref
      (:`Is Valid`
        (`/Game/Blueprints/CharacterStuff/BaseCharacter.EmoteNiceone` _characterref)))))

(event `InputAction|HappyEmote`
  (params (Key :type "Key Structure"))
  (bind _characterref (`self.CharacterRef`))
  ;[1 1 1] Emotes
  (:`Pressed`
    (`/Engine/EditorBlueprintResources/StandardMacros.IsValid` _characterref
      (:`Is Valid`
        (`/Game/Blueprints/CharacterStuff/BaseCharacter.Happy` _characterref)))))

(event `InputAction|wowEmote`
  (params (Key :type "Key Structure"))
  (bind _characterref (`self.CharacterRef`))
  ;[1 1 1] Emotes
  (:`Pressed`
    (`/Engine/EditorBlueprintResources/StandardMacros.IsValid` _characterref
      (:`Is Valid`
        (`/Game/Blueprints/CharacterStuff/BaseCharacter.EmoteWow` _characterref)))))

(event `InputAction|HahaEmote`
  (params (Key :type "Key Structure"))
  (bind _characterref (`self.CharacterRef`))
  ;[1 1 1] Emotes
  (:`Pressed`
    (`/Engine/EditorBlueprintResources/StandardMacros.IsValid` _characterref
      (:`Is Valid`
        (`/Game/Blueprints/CharacterStuff/BaseCharacter.HahaAnim` _characterref)))))

(event `GetMasterUIRef`
  (params (MasterUIWidget :type "/Game/Blueprints/UI/MasterUIWidget Object Reference"))
  (set `self.MasterUIWidget` MasterUIWidget))

(event `InputAxis|X-AxisMap`
  (params (AxisValue :type "Float (single-precision)"))
  (bind _characterref (`self.CharacterRef`))
  (`/Engine/EditorBlueprintResources/StandardMacros.IsValid` _characterref
    (:`Is Valid`
      (`/Game/Blueprints/CharacterStuff/BaseCharacter.X-AxisPassEvent` _characterref AxisValue))))

(event `Axis0`
  (bind _characterref (`self.CharacterRef`))
  (`/Engine/EditorBlueprintResources/StandardMacros.IsValid` _characterref
    (:`Is Valid`
      (`/Game/Blueprints/CharacterStuff/BaseCharacter.X-AxisPassEvent` _characterref 0.0)
      (`/Game/Blueprints/CharacterStuff/BaseCharacter.Y-AxisPassEvent` _characterref 0.0))))

(event `InputAxis|Y-Axis`
  (params (AxisValue :type "Float (single-precision)"))
  (bind _characterref (`self.CharacterRef`))
  (`/Engine/EditorBlueprintResources/StandardMacros.IsValid` _characterref
    (:`Is Valid`
      (`/Game/Blueprints/CharacterStuff/BaseCharacter.Y-AxisPassEvent` _characterref AxisValue))))

(event `InputAction|PauseMenu`
  (params (Key :type "Key Structure"))
  (:`Pressed`
    (`/Game/Blueprints/UI/MasterUIWidget.PauseMenuOpen` (`self.MasterUIWidget`))))

(event `InputAction|Interact`
  (params (Key :type "Key Structure"))
  (bind _characterref (`self.CharacterRef`))
  (:`Released`
    (`/Engine/EditorBlueprintResources/StandardMacros.IsValid` _characterref
      (:`Is Valid`
        (`/Game/Blueprints/CharacterStuff/BaseCharacter.InteractPassEvent` _characterref)))))

(event `InputAction|Use tool`
  (params (Key :type "Key Structure"))
  (bind _characterref (`self.CharacterRef`))
  (:`Pressed`
    (`/Engine/EditorBlueprintResources/StandardMacros.IsValid` _characterref
      (:`Is Valid`
        (if (not (`/Game/Blueprints/CharacterStuff/BaseCharacter.InMenu` _characterref))
          (`/Game/Blueprints/CharacterStuff/BaseCharacter.UseToolEvent` _characterref)))))
  (:`Released`
    (`/Engine/EditorBlueprintResources/StandardMacros.IsValid` _characterref
      (:`Is Valid`
        (`/Game/Blueprints/CharacterStuff/BaseCharacter.StopUsingToolEvent` _characterref)))))

(event `InputAction|Dash`
  (params (Key :type "Key Structure"))
  (:`Released`
    (`/Engine/EditorBlueprintResources/StandardMacros.DoOnce` false :!label _label
      (:`Completed`
        (`/Game/Blueprints/CharacterStuff/BaseCharacter.Dash Event Pass` (`self.CharacterRef`))
        (`KismetSystemLibrary.Delay` (`self.DashCooldown`))
        (goto _label :!via `Reset`)))))

(event `InputAction|Slap`
  (params (Key :type "Key Structure"))
  (bind _characterref (`self.CharacterRef`))
  (:`Released`
    (`/Engine/EditorBlueprintResources/StandardMacros.IsValid` _characterref
      (:`Is Valid`
        (`/Game/Blueprints/CharacterStuff/BaseCharacter.SlapEvent` _characterref)))))

(event `InputAction|Throw`
  (params (Key :type "Key Structure"))
  (:`Pressed`
    (bind _player_character_refrence (message `/Game/Blueprints/Interfaces/PlayerCharacterInterface/SolarSailorPlayerCharacterRefrenceGetter.Player Character Refrence Getter` (`self.K2_GetPawn`)))
    (`/Game/Blueprints/CharacterStuff/BaseCharacter.Throw own tool` _player_character_refrence)))

(event `InputAction|Pickup/Drop`
  (params (Key :type "Key Structure"))
  (:`Pressed`
    (bind _player_character_refrence (message `/Game/Blueprints/Interfaces/PlayerCharacterInterface/SolarSailorPlayerCharacterRefrenceGetter.Player Character Refrence Getter` (`self.K2_GetPawn`)))
    (`/Engine/EditorBlueprintResources/StandardMacros.IsValid` _player_character_refrence
      (:`Is Valid`
        (bind _tool_ref (message `/Game/Blueprints/Interfaces/ToolInterafce.Get tool Info` (`ChildActorComponent.ChildActor` (`/Game/Blueprints/CharacterStuff/BaseCharacter.EquippedTool` _player_character_refrence))))
        (if (`|EnumEquality` (`/Game/Blueprints/Tools/BP_BaseTool.What tool is this?` _tool_ref) "NewEnumerator0")
          (`/Game/Blueprints/CharacterStuff/BaseCharacter.Pick Up tool` _player_character_refrence)
          (else
            (`/Game/Blueprints/CharacterStuff/BaseCharacter.Drop Own Tool` _player_character_refrence)))))))

(fn `UserConstructionScript`)