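; Game mode for a two-player ship-hazard game that spawns characters at tagged PlayerStarts, initializes the camera and, outside TutorialLevel, starts hazard and level timers.
; A looping timer triggers a random eligible hazard, then totals damage by hazard type, ending the game if it exceeds ship health.
; When the level timer expires, damage relative to health sets a star rating.
; Countdown and result are only printed strings, with a Timeline refreshing the countdown.
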(event `self.ReceiveBeginPlay`
  (`self.GetPlayerStarts`)
  (`self.SpawnPlayers`)
  (bind _outactors (`GameplayStatics.GetAllActorsOfClass` "/Game/Blueprints/CharacterStuff/CameraBP.CameraBP_C"))
  (`/Game/Blueprints/CharacterStuff/CameraBP.InitialiseCamera` (`|GetArrayItem` _outactors))
  (bind _outactors_2 (`GameplayStatics.GetAllActorsOfClass` "/Game/Blueprints/HazardAssets/CoreHazardClass.CoreHazardClass_C"))
  (for _array_element _outactors_2
    (`KismetArrayLibrary.Array_AddUnique` (`self.Unsafe Hazard Refrences`) _array_element))
  (set `self.Hazard Max Index Range` (- (`KismetArrayLibrary.Array_Length` (`self.Unsafe Hazard Refrences`)) 1))
  (bind _returnvalue (`GameplayStatics.GetCurrentLevelName` true))
  (if (not (`KismetStringLibrary.EqualEqual_StrStr` _returnvalue "TutorialLevel"))
    (`self.Begin Trigger Activation Timer`)
    (`self.Start Game Timer`)))

(event `Begin Trigger Activation Timer`
  (bind _returnvalue (`KismetSystemLibrary.K2_SetTimerDelegate` (delegate `Hazard Trigger`) 5.0 true))
  (set `self.Hazard Trigger Timer` _returnvalue))

(event `Hazard Trigger`
  (`self.Activate Random Hazard`)
  (`self.CheckDamage`))

(event `Start Game Timer`
  (bind _returnvalue (`KismetSystemLibrary.K2_SetTimerDelegate` (delegate `Call Game End`) (`self.LevelTotalTime`)))
  (`Timeline|Timeline_0`
    (:`Update`
      (`KismetSystemLibrary.PrintString` (`KismetStringLibrary.Concat_StrStr` "Time Remaining:" " " (`KismetStringLibrary.Conv_IntToString` (`KismetMathLibrary.FTrunc` (`KismetSystemLibrary.K2_GetTimerRemainingTimeHandle` _returnvalue)))) true true (struct :`R` 0.045745 :`G` 1.0 :`A` 1.0) 0.0))))

(event `Call Game End`
  (bind _returnvalue (`KismetMathLibrary.MapRangeClamped` (`self.TotalDamage`) 0.0 (`self.ShipHealth`) 0.0 100.0))
  (`self.CheckDamage`)
  (if (<= _returnvalue 30.0)
    (`self.Call Level End` 3)
    (elif (<= _returnvalue 60.0)
      (`self.Call Level End` 2)
      (elif (<= _returnvalue 100.0)
        (`self.Call Level End` 1)
        (else
          (`self.Call Level End` 0 :!label _label))))))

(event `CallGameEndDestroyed`
  (goto _label))

(event `Call Level End`
  (params (Stars :type Integer))
  (`KismetSystemLibrary.PrintString` (`KismetStringLibrary.Concat_StrStr` "Game Over With:" " " (`KismetStringLibrary.Conv_IntToString` Stars) " Stars")))

(fn `Activate Random Hazard`
  (bind _returnvalue (`KismetMathLibrary.RandomIntegerInRange` 0 (- (`KismetArrayLibrary.Array_Length` (`self.Unsafe Hazard Refrences`)) 1)))
  ;[1 1 1] Find a random hazard that is currently susceptible to activation and activate it.
  (`KismetArrayLibrary.Array_Clear` (`self.Unsafe Hazard Refrences`))
  (bind _outactors (`GameplayStatics.GetAllActorsOfClass` "/Game/Blueprints/HazardAssets/CoreHazardClass.CoreHazardClass_C"))
  (for _array_element _outactors
    (if (`|EnumEquality` (`/Game/Blueprints/HazardAssets/CoreHazardClass.Hazard State` _array_element) "NewEnumerator1")
      (`KismetArrayLibrary.Array_AddUnique` (`self.Unsafe Hazard Refrences`) _array_element)))
  (if (`KismetArrayLibrary.Array_IsValidIndex` (`self.Unsafe Hazard Refrences`) _returnvalue)
    (`/Game/Blueprints/HazardAssets/CoreHazardClass.Trigger Recieved` (`|GetArrayItem` (`self.Unsafe Hazard Refrences`) _returnvalue))
    (else
      (`KismetSystemLibrary.K2_ClearAndInvalidateTimerHandle` (`self.Hazard Trigger Timer`))))
  (return))

(fn `CheckDamage`
  (if (> (`self.ShipHealth`) (`self.TotalDamage`))
    (set `self.TotalDamage` 0.0)
    (for _array_element (`self.Unsafe Hazard Refrences`)
      (if (`|EnumEquality` (`/Game/Blueprints/HazardAssets/CoreHazardClass.Hazard State` _array_element) "NewEnumerator2")
        (switch `/Game/Blueprints/HazardAssets/NatureOfHazard` (`/Game/Blueprints/HazardAssets/CoreHazardClass.Nature of Hazard` _array_element)
          (:`NewEnumerator4`
            (set `self.TotalDamage` (+ (`self.TotalDamage`) 5.0)))
          (:`NewEnumerator0`
            (set `self.TotalDamage` (+ (`self.TotalDamage`) 10.0)))
          (:`NewEnumerator3`
            (set `self.TotalDamage` (+ (`self.TotalDamage`) 15.0))))))
    (if (> (`self.TotalDamage`) (`self.ShipHealth`))
      (`self.CallGameEndDestroyed`))
    (else
      (`self.CallGameEndDestroyed`))))

(fn `Get Solar Sailor Object Refrence`
  (returns (`SS Gamemode Object Refrence` :type "/Game/Blueprints/GameMode/SSGamemode Object Reference"))
  (return self))

(fn `GetPlayerStarts`
  (bind _outactors (`GameplayStatics.GetAllActorsOfClass` "/Script/Engine.PlayerStart"))
  (set `self.PlayerStartArray` _outactors))

(fn `SpawnPlayers`
  (for _index (range 2)
    (set `self.IndexHold` _index)
    (for _array_element (`self.PlayerStartArray`)
      (if (== (`PlayerStart.PlayerStartTag` _array_element) (`KismetStringLibrary.Conv_StringToName` (`KismetStringLibrary.Conv_IntToString` (`self.IndexHold`))))
        (`GameplayStatics.CreatePlayer` (`self.IndexHold`))
        (bind _returnvalue (`|SpawnActorFromClass` "/Game/Blueprints/CharacterStuff/BaseCharacter.BaseCharacter_C" (`self.GetTransform` _array_element) "AlwaysSpawn" "OverrideRootScale" null null))
        (`Controller.Possess` (`GameplayStatics.GetPlayerController` (`self.IndexHold`)) _returnvalue)
        (`KismetArrayLibrary.Array_AddUnique` (`self.PlayersArray`) _returnvalue)))))

(fn `UserConstructionScript`)