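; SSGameInstance is a Game Instance Blueprint that tracks the stars earned per level and gates level loading.
; UpdateLevelStars writes a star count into the LevelStars array at the given level index.
; CheckIfCanLoadLevel always allows level index 0 and allows any later level only if the previous level has more than zero stars.
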(event `UpdateLevelStars`
  (params (LevelNum :type Integer) (NumberOfStars :type Integer))
  (`KismetArrayLibrary.Array_Set` (`self.LevelStars`) LevelNum NumberOfStars))

(fn `CheckIfCanLoadLevel`
  (params (LevelToCheck :type Integer))
  (returns (`CanLoad?` :type Boolean))
  (if (== LevelToCheck 0)
    (return true)
    (else
      (return (> (`|GetArrayItem` (`self.LevelStars`) (- LevelToCheck 1)) 0)))))