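; NatFunctionLibrary is a Blueprint function library that handles player deaths from hazards.
; PlayerCharacterDeathByHazard switches on hazard type, with Fire and Acid sharing one respawn path.
; It finds the killed actor in SSGamemode's PlayersArray and teleports it to the same-index PlayerStartArray location with zero rotation.
; An unconnected montage node, with no montage set, is noted as a possible place for an incineration animation.
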(fn `Player Character Death By Hazard`
  (params (`Hazard Type` :type "/Game/Blueprints/HazardAssets/NatureOfHazard Enum" :default "NewEnumerator0") (`Actor to kill` :type "/Game/Blueprints/CharacterStuff/BaseCharacter Object Reference"))
  (bind _asssgamemode (cast `/Game/Blueprints/GameMode/SSGamemode` (`GameplayStatics.GetGameMode` null) :!pure true))
  (switch `/Game/Blueprints/HazardAssets/NatureOfHazard` `Hazard Type`
    (:`NewEnumerator0`
      _)
    (:`NewEnumerator3`
      _))
  (for (_array_element _array_index) (`/Game/Blueprints/GameMode/SSGamemode.PlayersArray` _asssgamemode)
    (if (== `Actor to kill` _array_element)
      (`Actor.K2_TeleportTo` :`self` `Actor to kill` :`DestLocation` (`Actor.K2_GetActorLocation` (`|GetArrayItem` (`/Game/Blueprints/GameMode/SSGamemode.PlayerStartArray` _asssgamemode) _array_index))))))