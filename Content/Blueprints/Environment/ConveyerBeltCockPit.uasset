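; Cockpit conveyor belt actor that carries Food and characters overlapping its Box along the direction of its Forward component.
; Every Tick, it offsets overlapping Food by Speed and delta time without sweeping, regardless of IsMoving or belt direction.
; While IsMoving is set, it also pushes overlapping BaseCharacters through movement input scaled by DirectionScalar.
; The swapDirection event flips that scalar, so reversal affects only characters.
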(event `MovephysicsObj`
  (for _array_element (`PrimitiveComponent.GetOverlappingActors` (`self.Box`) null)
    (bind _asfood (cast `/Game/Blueprints/Environment/Food` _array_element))
    (`self.K2_AddActorWorldOffset` _asfood (* (`SceneComponent.GetForwardVector` (`self.Forward `)) (* (stale `self.ReceiveTick` DeltaSeconds) (`self.Speed`))) false false)))

(event `swap Direction`
  (set `self.DirectionScalar` (* -1 (`self.DirectionScalar`))))

(event `self.ReceiveTick`
  (params (DeltaSeconds :type "Float (single-precision)"))
  (`self.MovephysicsObj`)
  (if (`self.IsMoving`)
    (for _array_element (`PrimitiveComponent.GetOverlappingActors` (`self.Box`) null)
      (bind _asbase_character (cast `/Game/Blueprints/CharacterStuff/BaseCharacter` _array_element))
      (`Pawn.AddMovementInput` _asbase_character (* (`SceneComponent.GetForwardVector` (`self.Forward `)) (* DeltaSeconds (`self.Speed`))) (`self.DirectionScalar`) false))))

(fn `UserConstructionScript`)