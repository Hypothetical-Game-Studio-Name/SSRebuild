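; Timed door, named for the electric gun, that opens on an OpenDoor event and closes itself after TimeDoorOpen seconds.
; Opening shows a tick, turns two lights green and disables DoorBlock collision, while closing shows an exclamation point, turns them red and restores query-only collision.
; Helper functions only set Open and Closed flags, with no door movement here.
; FIsDoorOpen reads a separate IsDoorOpen variable that this graph never sets.
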(event `Open Door`
  (`SceneComponent.SetVisibility` (`self.Tick`) true false)
  (`SceneComponent.SetVisibility` (`self.Exclamation point `) false false)
  (`self.F_OpenDoor`)
  (`LightComponent.SetLightColor` (`self.Light1`) (struct :`R` 0.351533 :`G` 0.715693 :`B` 0.396755 :`A` 1.0) true)
  (`LightComponent.SetLightColor` (`self.Light2`) (struct :`R` 0.351533 :`G` 0.715693 :`B` 0.396755 :`A` 1.0) true)
  (`PrimitiveComponent.SetCollisionEnabled` (`self.DoorBlock`) "NoCollision")
  (`KismetSystemLibrary.K2_SetTimerDelegate` (delegate `ClosedDoor`) (`self.TimeDoorOpen`)))

(event `self.ReceiveBeginPlay`)

(event `ClosedDoor`
  (`SceneComponent.SetVisibility` (`self.Tick`) false false)
  (`SceneComponent.SetVisibility` (`self.Exclamation point `) true false)
  (`PrimitiveComponent.SetCollisionEnabled` (`self.DoorBlock`) "QueryOnly")
  (`self.F_CloseDoor`)
  (`LightComponent.SetLightColor` (`self.Light1`) (struct :`R` 1.0 :`G` 0.093059 :`B` 0.093059 :`A` 1.0) true)
  (`LightComponent.SetLightColor` (`self.Light2`) (struct :`R` 1.0 :`G` 0.093059 :`B` 0.093059 :`A` 1.0) true))

(fn `F_CloseDoor`
  (set `self.Open ` false)
  (set `self.Closed` true))

(fn `F_IsDoorOpen`
  (returns (IsDoorOpen :type Boolean))
  (if (`self.IsDoorOpen`)
    (return true)
    (else
      (return false))))

(fn `F_OpenDoor`
  (set `self.Open ` true))

(fn `UserConstructionScript`)