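; Automatic moving platform that shuttles back and forth between start and end marker components once play begins, if flagged active.
; BeginPlay caches both marker world locations and sets the play rate of two timelines from Duration and their start time from Newtime.
; The Towards and Backwards timelines lerp the actor's location without sweep, each handing off to the other through finish callbacks and a Return event for an endless loop.
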(event `self.ReceiveBeginPlay`
  ;[1 1 1] Move platform between a hidden in game mesh and its starting point
  (if (`self.ActivePlat`)
    (set `self.StartLoc` (`SceneComponent.K2_GetComponentLocation` (`self.PlatformStart `)))
    (set `self.EndLoc` (`SceneComponent.K2_GetComponentLocation` (`self.PlatformEnd`)))
    (`TimelineComponent.SetPlayRate` (`self.Towards`) (/ 1.0 (`self.Duration`)))
    (`TimelineComponent.SetPlayRate` (`self.Backwards`) (/ 1.0 (`self.Duration`)))
    (`TimelineComponent.SetNewTime` (`self.Backwards`) (`self.Newtime`))
    (`TimelineComponent.SetNewTime` (`self.Towards`) (`self.Newtime`))
    (bind (_direction _newtrack_0) (`Timeline|Towards` :!via `PlayFromStart` :!label _label)
      (:`Update`
        (`self.K2_SetActorLocation` (`KismetMathLibrary.VLerp` (`self.StartLoc`) (`self.EndLoc`) _newtrack_0)))
      (:`Finished`
        (bind (_direction_2 _newtrack_0_2) (`Timeline|Backwards` :!via `PlayFromStart`)
          (:`Update`
            (`self.K2_SetActorLocation` (`KismetMathLibrary.VLerp` (`self.StartLoc`) (`self.EndLoc`) _newtrack_0_2)))
          (:`Finished`
            (`self.Return`)))))))

(event `Return`
  ;[1 1 1] Move platform between a hidden in game mesh and its starting point
  (goto _label :!via `PlayFromStart`))

(fn `UserConstructionScript`)