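; BP_DoorWAnim is a door that opens when something overlaps its Box trigger and closes on a timer after the overlap ends.
; Opening sets Open, removes DoorBlock collision and turns both lights green; the DoorClosed timer event sets Closed, clears Open, restores query-only collision and turns them red.
; Separate open, close and query functions manage an IsDoorOpen flag that the event graph never uses.
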(event `self.ReceiveBeginPlay`)

(event `self.Box.OnComponentBeginOverlap`
  (params (OverlappedComponent :type "PrimitiveComponent Object Reference") (OtherActor :type "Actor Object Reference") (OtherComp :type "PrimitiveComponent Object Reference") (OtherBodyIndex :type Integer) (bFromSweep :type Boolean) (SweepResult :type "HitResult Structure (by ref)"))
  (set `self.Open` true)
  (`PrimitiveComponent.SetCollisionEnabled` (`self.DoorBlock`) "NoCollision")
  (`LightComponent.SetLightColor` (`self.Light2`) (struct :`R` 0.353054 :`G` 0.713542 :`B` 0.39555 :`A` 1.0) true)
  (`LightComponent.SetLightColor` (`self.Light1`) (struct :`R` 0.353054 :`G` 0.713542 :`B` 0.39555 :`A` 1.0) true))

(event `self.Box.OnComponentEndOverlap`
  (params (OverlappedComponent :type "PrimitiveComponent Object Reference") (OtherActor :type "Actor Object Reference") (OtherComp :type "PrimitiveComponent Object Reference") (OtherBodyIndex :type Integer))
  (`KismetSystemLibrary.K2_SetTimerDelegate` (delegate `DoorClosed`) (`self.Time Door is open for`)))

(event `DoorClosed`
  (set `self.Open` false)
  (set `self.Closed` true)
  (`PrimitiveComponent.SetCollisionEnabled` (`self.DoorBlock`) "QueryOnly")
  (`LightComponent.SetLightColor` (`self.Light2`) (struct :`R` 1.0 :`G` 0.093059 :`B` 0.093059 :`A` 1.0) true)
  (`LightComponent.SetLightColor` (`self.Light1`) (struct :`R` 1.0 :`G` 0.093059 :`B` 0.093059 :`A` 1.0) true))

(fn `F_CloseDoor`
  (bind _isdooropen (`self.F_IsDoorOpen`))
  (if _isdooropen
    (set `self.IsDoorOpen` false)))

(fn `F_IsDoorOpen`
  (returns (IsDoorOpen :type Boolean))
  (if (`self.IsDoorOpen`)
    (return true)
    (else
      (return false))))

(fn `F_OpenDoor`
  (bind _isdooropen (`self.F_IsDoorOpen`))
  (if (not _isdooropen)
    (set `self.IsDoorOpen` true)))

(fn `UserConstructionScript`)