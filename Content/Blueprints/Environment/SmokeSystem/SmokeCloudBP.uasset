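; Smoke cloud actor that thickens or clears over time and stops the player sprinting while it is full.
; SmokeTimer plays a timeline, first setting its time if the new value is below LastTimeToFull, and ClearSmoke reverses it.
; The timeline drives opacity on a construction-time dynamic material and toggles RestrictDash when finished.
; Box overlap disables CanSprint while restricted; leaving restores it, but clearing alone does not.
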(event `SmokeTimer`
  (params (NewTimeToFull :type "Float (double-precision)"))
  (if (< NewTimeToFull (`self.LastTimeToFull`))
    (`|ExecutionSequence`
      (:`then_0`
        (bind (_direction _smokealpha) (`Timeline|SmokeTimeline` :`NewTime` NewTimeToFull :!via `SetNewTime` :!label _label)
          (:`Update`
            (bind _output_get (set `self.SmokeBind` _smokealpha))
            (`MaterialInstanceDynamic.SetScalarParameterValue` (`self.SmokeMaterial`) "OpacityParameter" _output_get))
          (:`Finished`
            (switch `ETimelineDirection` _direction
              (:`Forward`
                (set `self.RestrictDash?` true)
                (`self.Check If smoke if somke hinders movement`))
              (:`Backward`
                (set `self.RestrictDash?` false))))))
      (:`then_1`
        (goto _label)))
    (else
      (goto _label))))

(event `ClearSmoke`
  (goto _label :!via `Reverse`))

(event `self.Box.OnComponentBeginOverlap`
  (params (OverlappedComponent :type "PrimitiveComponent Object Reference") (OtherActor :type "Actor Object Reference") (OtherComp :type "PrimitiveComponent Object Reference") (OtherBodyIndex :type Integer) (bFromSweep :type Boolean) (SweepResult :type "HitResult Structure (by ref)"))
  (bind _player_character_refrence (message `/Game/Blueprints/Interfaces/PlayerCharacterInterface/SolarSailorPlayerCharacterRefrenceGetter.Player Character Refrence Getter` OtherActor))
  (`/Engine/EditorBlueprintResources/StandardMacros.IsValid` _player_character_refrence
    (:`Is Valid`
      (`self.Check If smoke if somke hinders movement`))))

(event `Check If smoke if somke hinders movement`
  (`/Engine/EditorBlueprintResources/StandardMacros.IsValid` (stale `self.Box.OnComponentBeginOverlap` _player_character_refrence)
    (:`Is Valid`
      (if (`self.RestrictDash?`)
        (set `/Game/Blueprints/CharacterStuff/BaseCharacter.Can Sprint?` false (stale `self.Box.OnComponentBeginOverlap` _player_character_refrence))))))

(event `self.Box.OnComponentEndOverlap`
  (params (OverlappedComponent :type "PrimitiveComponent Object Reference") (OtherActor :type "Actor Object Reference") (OtherComp :type "PrimitiveComponent Object Reference") (OtherBodyIndex :type Integer))
  (bind _player_character_refrence (message `/Game/Blueprints/Interfaces/PlayerCharacterInterface/SolarSailorPlayerCharacterRefrenceGetter.Player Character Refrence Getter` OtherActor))
  (`/Engine/EditorBlueprintResources/StandardMacros.IsValid` _player_character_refrence
    (:`Is Valid`
      (set `/Game/Blueprints/CharacterStuff/BaseCharacter.Can Sprint?` true _player_character_refrence))))

(fn `UserConstructionScript`
  (bind _returnvalue (`KismetMaterialLibrary.CreateDynamicMaterialInstance` "/Game/Blueprints/Environment/SmokeSystem/SmokeMaterial.SmokeMaterial"))
  (`MaterialInstanceDynamic.SetScalarParameterValue` _returnvalue "OpacityParameter" (`self.SmokeBind`))
  (`PrimitiveComponent.SetMaterial` (`self.SmokeMesh`) 0 _returnvalue)
  (set `self.SmokeMaterial` _returnvalue))