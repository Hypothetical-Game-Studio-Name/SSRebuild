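; Conveyor belt actor that pushes whatever actors overlap its Box while IsMoving is set.
; Each Tick, it offsets those actors along the Forward component's forward vector, scaled by Speed and delta time, without sweeping.
; The world-space direction is applied as a local offset, so each actor's own rotation alters the direction it travels.
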(event `self.ReceiveBeginPlay`)

(event `self.ReceiveTick`
  (params (DeltaSeconds :type "Float (single-precision)"))
  (`|ExecutionSequence`
    (:`then_0`
      (if (`self.IsMoving`)
        (for _array_element (`PrimitiveComponent.GetOverlappingActors` (`self.Box`) null)
          (`self.K2_AddActorLocalOffset` _array_element (* (`SceneComponent.GetForwardVector` (`self.Forward `)) (* DeltaSeconds (`self.Speed`))) false false))))
    (:`then_1`
      (if true
        _))))

(fn `UserConstructionScript`)