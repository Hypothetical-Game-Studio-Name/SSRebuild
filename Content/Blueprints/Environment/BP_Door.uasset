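; Door Blueprint that switches between open and closed states in response to bound open and close events.
; On BeginPlay it binds OpenDoor and CloseDoor, which call functions that check IsDoorOpen to skip redundant changes.
; These functions only set boolean flags as a temporary stand-in for animation, with closing also setting Closed to false.
; The OpeningDoor event is an empty stub.
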(event `OpeningDoor`)

(event `Open Door`
  (`self.F_OpenDoor`))

(event `self.ReceiveBeginPlay`
  (add `self.OpenDoor` (delegate `Open Door`))
  (add `self.CloseDoor` (delegate `Close Door`)))

(event `Close Door`
  (`self.F_CloseDoor`))

(fn `F_CloseDoor`
  (bind _isdooropen (`self.F_IsDoorOpen`))
  (if _isdooropen
    ;[1 1 1] Temp - replace with animation
    (set `self.IsDoorOpen` false)
    (set `self.Open ` false)
    (set `self.Closed` false)))

(fn `F_IsDoorOpen`
  (returns (IsDoorOpen :type Boolean))
  (if (`self.IsDoorOpen`)
    (return true)
    (else
      (return false))))

(fn `F_OpenDoor`
  (bind _isdooropen (`self.F_IsDoorOpen`))
  (if (not _isdooropen)
    (set `self.IsDoorOpen` true)
    ;[1 1 1] Temp - replace with animation
    (set `self.Open ` true)))

(fn `UserConstructionScript`)