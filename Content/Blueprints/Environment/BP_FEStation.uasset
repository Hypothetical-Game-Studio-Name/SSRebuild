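; BP_FEStation is a fire extinguisher dock meant to recharge the extinguisher held as its FEDockPoint child actor.
; While docked, Tick casts to BP_FireExtinguisher and updates BatteryLife if above zero, though the increment is currently multiplied by zero.
; The charge display gets a new dynamic material each update, with green driven by BatteryLife.
; A test-only overlap event undocks by clearing the child actor class.
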(event `self.ReceiveTick`
  (params (DeltaSeconds :type "Float (single-precision)"))
  (bind _isfireextinguisherdocked (`self.F_IsFireExtinguisherDocked`))
  (if _isfireextinguisherdocked
    (`self.F_ChargeFireExtinguisher` (`GameplayStatics.GetTimeSeconds`))))

(event `self.ReceiveActorBeginOverlap`
  (params (OtherActor :type "Actor Object Reference"))
  ;[1 1 1] For TESTING ONLY
  (`self.F_UndockFireExtinguisher`))

(fn `F_ChargeAmountDisplay `
  (params (ChargeAmount :type "Float (double-precision)"))
  (locals (ChargeAmountDisplayMaterial :type "MaterialInstanceDynamic Object Reference"))
  (bind _returnvalue (`PrimitiveComponent.CreateDynamicMaterialInstance` (`self.ChargeAmountDisplay`) 0 "/Game/Materials/Mat_FEChargeAmountDisplay.Mat_FEChargeAmountDisplay" "None"))
  (bind _output_get (set `local.ChargeAmountDisplayMaterial` _returnvalue))
  (`MaterialInstanceDynamic.SetVectorParameterValue` _output_get "Base Color" (`KismetMathLibrary.MakeColor` 0.0 ChargeAmount 0.0 0.5)))

(fn `F_ChargeFireExtinguisher`
  (params (Seconds :type "Float (double-precision)"))
  ;[1 1 1] !! Change to Interface
  (bind _asbp_fire_extinguisher (cast `/Game/Blueprints/Tools/BP_FireExtinguisher` (`ChildActorComponent.ChildActor` (`self.FE_DockPoint`))))
  (bind _batterylife (`/Game/Blueprints/Tools/BP_BaseTool.BatteryLife` _asbp_fire_extinguisher))
  (if (< 0.0 _batterylife)
    (bind _output_get (set `/Game/Blueprints/Tools/BP_BaseTool.BatteryLife` (+ _batterylife (* 0 (`self.BatteryChargeMultiplier`))) _asbp_fire_extinguisher))
    (`self.F_ChargeAmountDisplay ` _output_get)
    (`KismetSystemLibrary.PrintString` (`KismetStringLibrary.Concat_StrStr` "Battery is at:" (`KismetStringLibrary.Conv_DoubleToString` 0.0) "%"))))

(fn `F_IsFireExtinguisherDocked`
  (returns (IsFireExtinguisherDocked :type Boolean))
  (if (== (`ChildActorComponent.ChildActorClass` (`self.FE_DockPoint`)) "/Game/Blueprints/Tools/BP_FireExtinguisher.BP_FireExtinguisher_C")
    (return true)
    (else
      (return false))))

(fn `F_UndockFireExtinguisher`
  (bind _isfireextinguisherdocked (`self.F_IsFireExtinguisherDocked`))
  (if _isfireextinguisherdocked
    (`ChildActorComponent.SetChildActorClass` (`self.FE_DockPoint`) null)))

(fn `UserConstructionScript`)