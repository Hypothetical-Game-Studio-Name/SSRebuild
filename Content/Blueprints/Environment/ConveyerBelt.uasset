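; Conveyor belt actor that carries overlapping physics objects along its surface and can reverse direction.
; While moving, Tick offsets physics-collision components overlapping PhysicsApplication along the belt direction, scaled by Speed and frame time.
; swapDirection toggles visibility of the forward and backward meshes and rotates the direction vector 180 degrees.
; The construction script creates a dynamic material on the forward mesh to derive its scroll speed from Speed.
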(event `self.ReceiveBeginPlay`
  (set `self.Conveyor Belt Direction` (`SceneComponent.GetForwardVector` (`self.Backward Mesh`))))

(event `swap Direction`
  (bind _returnvalue (`KismetMathLibrary.GreaterGreater_VectorRotator` (`self.Conveyor Belt Direction`) (struct :`Yaw` 180.0)))
  (`/Engine/EditorBlueprintResources/StandardMacros.FlipFlop`
    (:`A`
      (`SceneComponent.ToggleVisibility` (`self.Forwards Mesh`) false)
      (`SceneComponent.ToggleVisibility` (`self.Backward Mesh`) false)
      (set `self.Conveyor Belt Direction` _returnvalue))
    (:`B`
      (`SceneComponent.ToggleVisibility` (`self.Backward Mesh`) false)
      (`SceneComponent.ToggleVisibility` (`self.Forwards Mesh`) false)
      (set `self.Conveyor Belt Direction` _returnvalue))))

(event `self.ReceiveTick`
  (params (DeltaSeconds :type "Float (single-precision)"))
  (if (`self.IsMoving`)
    (for _array_element (`PrimitiveComponent.GetOverlappingComponents` (`self.Physics Application`))
      (if (`PrimitiveComponent.K2_IsPhysicsCollisionEnabled` _array_element)
        (`SceneComponent.K2_AddWorldOffset` _array_element (* (`self.Conveyor Belt Direction`) (* DeltaSeconds (`self.Speed`))) false false)))))

(fn `UserConstructionScript`
  (set `self.BeltSpeedMult` (* (/ (`self.Speed`) 136.0) 1.1))
  (bind _returnvalue (`PrimitiveComponent.CreateDynamicMaterialInstance` (`self.Forwards Mesh`) 1 "/Game/ArtFolder/Art/Materials/Environment/ConveyorBelt/Belt.Belt" "None"))
  (bind _output_get (set `self.BeltMat` _returnvalue))
  (`MaterialInstanceDynamic.SetScalarParameterValue` _output_get "BeltSpeed" (* (`self.BeltSpeedMult`) -0.05)))