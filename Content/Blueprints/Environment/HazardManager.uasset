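; HazardManager is a level hazard controller that sets off random environmental hazards on a repeating timer.
; On BeginPlay it caches every actor of CoreHazardClass in HazardArray, then starts the BeginCreations event.
; BeginCreations loops endlessly through a Delay of DelayDuration, calling TriggerRecieved on a randomly indexed hazard after each wait.
; The array is gathered only once, and the same hazard can be picked on consecutive cycles.
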(event `self.ReceiveBeginPlay`
  (bind _outactors (`GameplayStatics.GetAllActorsOfClass` "/Game/Blueprints/HazardAssets/CoreHazardClass.CoreHazardClass_C"))
  (set `self.HazardArray` _outactors)
  (`self.BeginCreations`))

(event `BeginCreations`
  (bind _hazardarray (`self.HazardArray`))
  (`KismetSystemLibrary.Delay` (`self.DelayDuration`) :!label _label)
  (`/Game/Blueprints/HazardAssets/CoreHazardClass.Trigger Recieved` (`|GetArrayItem` _hazardarray (`KismetMathLibrary.RandomIntegerInRange` 0 (- (`KismetArrayLibrary.Array_Length` _hazardarray) 1))))
  (goto _label))

(fn `UserConstructionScript`)