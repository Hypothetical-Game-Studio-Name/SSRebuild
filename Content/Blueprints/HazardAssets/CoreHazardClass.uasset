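; Core hazard actor for breach, fire, acid and flame-vent (Electric) hazards, moving between safe, unsafe and active states.
; Triggers arm then activate it, showing its marker and starting either timed evolution (breach→fire→acid) or timeline-driven flame bursts.
; Matching tool projectiles drain its health until safe, optionally starting a re-trigger timer, while reinforced plating seals it.
; Active fires and vents burn, then incinerate overlapping players through timers cleared on exit.
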(event `self.ReceiveBeginPlay`
  ;[1 1 1] Set hazard marker variable
  (bind _ashazard_marker (cast `/Game/Blueprints/HazardAssets/HazardUI/HazardMarker` (`WidgetComponent.GetUserWidgetObject` (`self.Hazard Widget`))))
  (set `self.HazardMarkerVar` _ashazard_marker)
  (`/Game/Blueprints/HazardAssets/HazardUI/HazardMarker.SetHazardBrush` (`self.HazardMarkerVar`) (`self.Nature of Hazard`)))

(event `Hazard Progress`
  ;[1 1 1] If the hazard progresses, this is the blueprint that handles the changing of the 'hazard nature'
  (if (`self.Does Hazard Evolve?`)
    (bind _returnvalue (`KismetSystemLibrary.K2_SetTimerDelegate` (delegate `Hazard Evolve`) 10.0 true))
    (set `self.Hazard Progression Timer` _returnvalue)))

(event `Hazard saftey timer`
  ;[0.03179 1 0] Step 1. Hazard is either activated, made unsafe, or made worse.
  (if (`self.One Time Hazard?`)
    (`KismetSystemLibrary.PrintString` "GOGO")
    (bind _returnvalue (`KismetSystemLibrary.K2_SetTimerDelegate` (delegate `Trigger Recieved`) 5.0))
    (set `self.Hazard Saftey Timer Handle` _returnvalue)))

(event `Hazard Evolve`
  (bind _hazardeffect (`self.HazardEffect`))
  ;[1 1 1] If the hazard progresses, this is the blueprint that handles the changing of the 'hazard nature'
  (switch `/Game/Blueprints/HazardAssets/NatureOfHazard` (`self.Nature of Hazard`)
    (:`NewEnumerator4`
      (`ParticleSystemComponent.SetTemplate` _hazardeffect "/Game/StarterContent/Particles/P_Fire.P_Fire")
      (bind _output_get (set `self.Nature of Hazard` "NewEnumerator0"))
      (`/Game/Blueprints/HazardAssets/HazardUI/HazardMarker.SetHazardBrush` (`self.HazardMarkerVar`) _output_get))
    (:`NewEnumerator0`
      (`ParticleSystemComponent.SetTemplate` _hazardeffect "/Game/StarterContent/Particles/P_Sparks.P_Sparks")
      (bind _output_get_2 (set `self.Nature of Hazard` "NewEnumerator3"))
      (`/Game/Blueprints/HazardAssets/HazardUI/HazardMarker.SetHazardBrush` (`self.HazardMarkerVar`) _output_get_2))))

(event `Trigger Recieved`
  (bind _hazardeffect (`self.HazardEffect`))
  ;[0.03179 1 0] Step 1. Hazard is either activated, made unsafe, or made worse.
  (`KismetSystemLibrary.PrintString` "TRIGGER")
  (`KismetSystemLibrary.PrintString` (`|GetEnumeratorNameAsString` (`self.Nature of Hazard`)))
  (switch `/Game/Blueprints/HazardAssets/HazardState` (`self.Hazard State`)
    (:`NewEnumerator0`
      (set `self.Hazard State` "NewEnumerator1")
      (set `self.Hazard Health` 100.0)
      (bind _output_get (set `self.Nature of Hazard` (`self.Hazard Base Nature`)))
      (switch `/Game/Blueprints/HazardAssets/NatureOfHazard` _output_get
        (:`NewEnumerator4`
          (`ParticleSystemComponent.SetTemplate` (`self.HazardEffect`) "/Game/StarterContent/Particles/P_Smoke.P_Smoke"))
        (:`NewEnumerator0`
          (`ParticleSystemComponent.SetTemplate` _hazardeffect "/Game/ArtFolder/Particles/M5VFXVOL2/Particles/Fire/Fire_03.Fire_03"))
        (:`NewEnumerator3`
          (`ParticleSystemComponent.SetTemplate` _hazardeffect "/Game/StarterContent/Particles/P_Sparks.P_Sparks"))))
    (:`NewEnumerator1`
      (`self.Hazard Activated`))))

(event `self.Fix Range.OnComponentBeginOverlap`
  (params (OverlappedComponent :type "PrimitiveComponent Object Reference") (OtherActor :type "Actor Object Reference") (OtherComp :type "PrimitiveComponent Object Reference") (OtherBodyIndex :type Integer) (bFromSweep :type Boolean) (SweepResult :type "HitResult Structure (by ref)"))
  ;[1 1 1] When the hazard is hit with a projectile, this determines wether or not it actually gets repair damage.
  (if (`|EnumEquality` (`self.Hazard State`) "NewEnumerator2")
    (bind _astool_projectile_master (cast `/Game/Blueprints/Tools/Projectiles/ToolProjectileMaster` OtherActor))
    (bind _which_hazard_does_this_fix (`/Game/Blueprints/Tools/Projectiles/ToolProjectileMaster.Which hazard does this fix` _astool_projectile_master))
    (switch `/Game/Blueprints/HazardAssets/NatureOfHazard` _which_hazard_does_this_fix
      (:`NewEnumerator4`
        (bind _returnvalue (`|EnumEquality` (`self.Nature of Hazard`) _which_hazard_does_this_fix))
        (if _returnvalue
          (`self.Repair Breach`)))
      (:`NewEnumerator0`
        (if _returnvalue
          (`self.Extinguish Fire Hazard`)))
      (:`NewEnumerator3`
        (if _returnvalue
          (`self.Repair Acidic Damage`))))))

(event `/Game/Blueprints/Interfaces/InteractEvent.Is interacted with`
  (params (`Character who interacts` :type "/Game/Blueprints/CharacterStuff/BaseCharacter Object Reference"))
  (bind _equippedtool (`/Game/Blueprints/CharacterStuff/BaseCharacter.EquippedTool` `Character who interacts`))
  ;[1 1 1] This is for when the hazard recieves reinforced plating
  (if (== (`ChildActorComponent.ChildActorClass` _equippedtool) "/Game/Blueprints/HazardAssets/Reinforced_Plating/ReinforcedPlating.ReinforcedPlating_C")
    (`ChildActorComponent.SetChildActorClass` _equippedtool "/Game/Blueprints/Tools/BP_HammerTool.BP_HammerTool_C")
    (`SceneComponent.SetVisibility` (`self.Plating Mesh`) true false)
    (`ActorComponent.Deactivate` (`self.HazardEffect`))
    (`self.Clear Timers`)
    (set `self.Hazard State` "NewEnumerator0")))

(event `Flame Vent Begin Activity`
  ;[1 1 1] When this hazard is a flame vent, this controls the flames shooting outward
  (`KismetSystemLibrary.K2_SetTimerDelegate` (delegate `Shoot Fire`) 3.0 :!label _label))

(event `Vent Cooldown`
  ;[1 1 1] When this hazard is a flame vent, this controls the flames shooting outward
  (goto _label))

(event `Extinguish Fire Hazard`
  ;[1 1 1] This fires if hit by extinguisher foam
  (bind _output_get (set `self.Hazard Health` (- (`self.Hazard Health`) 10.0)))
  (`KismetSystemLibrary.PrintString` (`KismetStringLibrary.Conv_DoubleToString` _output_get) true true (struct :`R` 1.0 :`G` 0.003511 :`A` 1.0))
  (if (<= _output_get 0.0)
    (`ActorComponent.Deactivate` (`self.HazardEffect`))
    (set `self.Hazard State` "NewEnumerator0")
    (`self.Hazard saftey timer`)
    (`/Game/Blueprints/HazardAssets/HazardUI/HazardMarker.HideHazardMarker` (`self.HazardMarkerVar`))))

(event `Shoot Fire`
  (bind _returnvalue (`self.K2_GetActorLocation`))
  (bind _hazardeffectapplyrange (`self.HazardEffectApplyRange`))
  (bind (_normal_range_x _normal_range_y _normal_range_z) (`KismetMathLibrary.BreakVector` (`self.Normal Range`)))
  (bind (_returnvalue_x _returnvalue_y _returnvalue_z) (`KismetMathLibrary.BreakVector` (`SceneComponent.K2_GetComponentLocation` _hazardeffectapplyrange)))
  ;[1 1 1] When this hazard is a flame vent, this controls the flames shooting outward
  (set `self.Normal Range` (`BoxComponent.BoxExtent` (`self.HazardEffectApplyRange`)))
  (bind (_direction _flame_alpha _box_extension) (`Timeline|FlameShot` :!via `PlayFromStart`)
    (:`Update`
      (`SceneComponent.K2_SetWorldLocation` _hazardeffectapplyrange (`KismetMathLibrary.MakeVector` (.x (`KismetMathLibrary.VLerp` _returnvalue (+ _returnvalue (* (`self.GetActorForwardVector`) 100.0)) _flame_alpha)) (.y (`KismetMathLibrary.VLerp` _returnvalue (+ _returnvalue (* (`self.GetActorForwardVector`) 100.0)) _flame_alpha)) _returnvalue_z) false false)
      (`BoxComponent.SetBoxExtent` (`self.HazardEffectApplyRange`) (`KismetMathLibrary.MakeVector` _normal_range_x _normal_range_y (+ _normal_range_z _box_extension)) true))
    (:`Finished`
      (`self.Vent Cooldown`))))

(event `Repair Breach`
  ;[1 1 1] This fires if hit by hammer repair orb
  (bind _output_get (set `self.Hazard Health` (- (`self.Hazard Health`) 10.0)))
  (`KismetSystemLibrary.PrintString` (`KismetStringLibrary.Conv_DoubleToString` _output_get) true true (struct :`R` 1.0 :`G` 0.003511 :`A` 1.0))
  (if (<= _output_get 0.0)
    (`ActorComponent.Deactivate` (`self.HazardEffect`))
    (set `self.Hazard State` "NewEnumerator0")
    (`self.Hazard saftey timer`)
    (`/Game/Blueprints/HazardAssets/HazardUI/HazardMarker.HideHazardMarker` (`self.HazardMarkerVar`))))

(event `Repair Acidic Damage`
  ;[1 1 1] This fires if hit by electric repair bullet.
  (bind _output_get (set `self.Hazard Health` (- (`self.Hazard Health`) 10.0)))
  (`KismetSystemLibrary.PrintString` (`KismetStringLibrary.Conv_DoubleToString` _output_get) true true (struct :`R` 1.0 :`G` 0.003511 :`A` 1.0))
  (if (<= _output_get 0.0)
    (`ActorComponent.Deactivate` (`self.HazardEffect`))
    (set `self.Hazard State` "NewEnumerator0")
    (`self.Hazard saftey timer`)
    (`/Game/Blueprints/HazardAssets/HazardUI/HazardMarker.HideHazardMarker` (`self.HazardMarkerVar`))))

(event `self.HazardEffectApplyRange.OnComponentBeginOverlap`
  (params (OverlappedComponent :type "PrimitiveComponent Object Reference") (OtherActor :type "Actor Object Reference") (OtherComp :type "PrimitiveComponent Object Reference") (OtherBodyIndex :type Integer) (bFromSweep :type Boolean) (SweepResult :type "HitResult Structure (by ref)"))
  ;[1 0.3958 0.3958] If the hazard is a fire, and IS ACTIVE, These nodes handle setting any player character that walks into the applicable range of the fire, on fire.
  (switch `/Game/Blueprints/HazardAssets/NatureOfHazard` (`self.Nature of Hazard`)
    (:`NewEnumerator0`
      (if (`|EnumEquality` (`self.Hazard State`) "NewEnumerator2")
        (bind _player_character_refrence (message `/Game/Blueprints/Interfaces/PlayerCharacterInterface/SolarSailorPlayerCharacterRefrenceGetter.Player Character Refrence Getter` OtherActor))
        (`/Engine/EditorBlueprintResources/StandardMacros.IsValid` _player_character_refrence
          (:`Is Valid`
            (set `self.Character To Effect` _player_character_refrence)
            (bind _returnvalue (`KismetSystemLibrary.K2_SetTimerDelegate` (delegate `Burn Player Character`) (`self.Time to Burn Character`)))
            (bind _output_get (set `self.Apply Player Burn Timer` _returnvalue))
            (`KismetArrayLibrary.Array_AddUnique` (`self.Fire Timers`) _output_get)
            (bind _returnvalue_2 (`KismetSystemLibrary.K2_SetTimerDelegate` (delegate `Incinerate Player Character`) (`self.Time to Incinerate Character`) :!label _label_2))
            (bind _output_get_2 (set `self.Player Kill Timer` _returnvalue_2))
            (`KismetArrayLibrary.Array_AddUnique` (`self.Fire Timers`) _output_get_2)))))
    (:`NewEnumerator7`
      ;[1 1 1] If the hazard happens to be a flame vent, the burning effect is instantenously applied to the player character
      (if (`|EnumEquality` (`self.Hazard State`) "NewEnumerator2")
        (`self.Burn Player Character`)
        (goto _label_2)))))

(event `Burn Player Character`
  ;[1 0.3958 0.3958] If the hazard is a fire, and IS ACTIVE, These nodes handle setting any player character that walks into the applicable range of the fire, on fire.
  (bind _player_character_refrence (message `/Game/Blueprints/Interfaces/PlayerCharacterInterface/SolarSailorPlayerCharacterRefrenceGetter.Player Character Refrence Getter` (stale `self.HazardEffectApplyRange.OnComponentBeginOverlap` OtherActor)))
  (`/Engine/EditorBlueprintResources/StandardMacros.IsValid` _player_character_refrence
    (:`Is Valid`
      (bind _output_get (set `self.Character To Effect` _player_character_refrence))
      (if (not (`self.Is player already on fire?` (`/Game/Blueprints/CharacterStuff/BaseCharacter.Hazard Effect` (`self.Character To Effect`))))
        (`ParticleSystemComponent.SetTemplate` (`/Game/Blueprints/CharacterStuff/BaseCharacter.Hazard Effect` (`self.Character To Effect`)) "/Game/StarterContent/Particles/P_Fire.P_Fire"))
      (`/Game/Blueprints/CharacterStuff/BaseCharacter.Taking Hazard Effect` _output_get "NewEnumerator0"))))

(event `Incinerate Player Character`
  ;[1 0.3958 0.3958] If the hazard is a fire, and IS ACTIVE, These nodes handle setting any player character that walks into the applicable range of the fire, on fire.
  (`/Game/Blueprints/CharacterStuff/BaseCharacter.Hazard Death Event` (`self.Character To Effect`) "NewEnumerator0"))

(event `self.HazardEffectApplyRange.OnComponentEndOverlap`
  (params (OverlappedComponent :type "PrimitiveComponent Object Reference") (OtherActor :type "Actor Object Reference") (OtherComp :type "PrimitiveComponent Object Reference") (OtherBodyIndex :type Integer))
  ;[1 0.3958 0.3958] If the hazard is a fire, and IS ACTIVE, These nodes handle setting any player character that walks into the applicable range of the fire, on fire.
  ;;[1 1 1] The player character can step out of the flames, to prevent themselves from getting burned, or incinerated.
  (`/Engine/EditorBlueprintResources/StandardMacros.IsValid` OtherActor
    (:`Is Valid`
      (bind _player_character_refrence (message `/Game/Blueprints/Interfaces/PlayerCharacterInterface/SolarSailorPlayerCharacterRefrenceGetter.Player Character Refrence Getter` OtherActor))
      (`/Engine/EditorBlueprintResources/StandardMacros.IsValid` _player_character_refrence
        (:`Is Valid`
          (for _array_element (`self.Fire Timers`)
            (`KismetSystemLibrary.K2_ClearAndInvalidateTimerHandle` _array_element)))))))

(fn `Clear Timers`
  (`KismetSystemLibrary.K2_ClearAndInvalidateTimerHandle` (`self.Hazard Saftey Timer Handle`))
  (`KismetSystemLibrary.K2_ClearAndInvalidateTimerHandle` (`self.Hazard Progression Timer`))
  (`KismetSystemLibrary.K2_ClearAndInvalidateTimerHandle` (`self.Apply Player Burn Timer`))
  (`KismetSystemLibrary.K2_ClearAndInvalidateTimerHandle` (`self.Hazard Saftey Timer Handle`))
  (return))

(fn `Hazard Activated`
  (bind (_returnvalue_location _returnvalue_rotation _returnvalue_scale) (`KismetMathLibrary.BreakTransform` (`SceneComponent.K2_GetComponentToWorld` (`self.HazardEffectApplyRange`))))
  ;[1 1 1] Step 2. Hazard is activated, the hazard type is then created
  (set `self.Worst Hazard State Damage Multiplier` 0)
  (`GameplayStatics.SpawnEmitterAtLocation` "/Game/StarterContent/Particles/P_Explosion.P_Explosion" _returnvalue_location _returnvalue_rotation _returnvalue_scale)
  (set `self.Hazard State` "NewEnumerator2")
  (`ActorComponent.Activate` (`self.HazardEffect`) false)
  (`/Game/Blueprints/HazardAssets/HazardUI/HazardMarker.ShowHazardMarker` (`self.HazardMarkerVar`))
  (switch `/Game/Blueprints/HazardAssets/NatureOfHazard` (`self.Nature of Hazard`)
    (:`NewEnumerator4`
      (`self.Hazard Progress` :!label _label))
    (:`NewEnumerator0`
      (goto _label))
    (:`NewEnumerator3`
      (goto _label))
    (:`NewEnumerator7`
      (`self.Flame Vent Begin Activity`))))

(fn `Hazard is repaired`
  (`ActorComponent.Deactivate` (`self.HazardEffect`))
  (set `self.Hazard State` "NewEnumerator0"))

(fn `Increase Severity`
  ;[1 1 1] Step 3. Severity is Increased
  (switch `/Game/Blueprints/HazardAssets/HazardSeverity` (`self.How Severe is the hazard?`)
    (:`NewEnumerator0`
      (set `self.How Severe is the hazard?` "NewEnumerator1"))
    (:`NewEnumerator1`
      (set `self.How Severe is the hazard?` "NewEnumerator2"))
    (:`NewEnumerator2`
      (`/Engine/EditorBlueprintResources/StandardMacros.IncrementInt` (`self.Worst Hazard State Damage Multiplier`)
        (:`  `
          _))))
  (return))

(fn `Is player already on fire?`
  (params (`Hazard Effect Input` :type "ParticleSystemComponent Object Reference"))
  (returns (Result :type Boolean))
  (return (== (`ParticleSystemComponent.Template` `Hazard Effect Input`) "/Game/StarterContent/Particles/P_Fire.P_Fire")))

(fn `Set Severity`
  ;[1 1 1] This visually reflects the current severity of the hazard
  (switch `/Game/Blueprints/HazardAssets/HazardSeverity` (`self.How Severe is the hazard?`)
    (:`NewEnumerator0`
      (`SceneComponent.SetRelativeScale3D` (`self.HazardEffect`) (0.3 0.3 0.3))
      (return))
    (:`NewEnumerator1`
      (`SceneComponent.SetRelativeScale3D` (`self.HazardEffect`) (1.0 1.0 1.0))
      (return))
    (:`NewEnumerator2`
      (return))))

(fn `Small Breach Repair Event`)

(fn `Small Fire has started`)

(fn `Small Fire Hazard Repair Event`
  (params (`Character Input` :type "/Game/Blueprints/CharacterStuff/BaseCharacter Object Reference"))
  (if (== (`ChildActorComponent.ChildActorClass` (`/Game/Blueprints/CharacterStuff/BaseCharacter.EquippedTool` `Character Input`)) (`self.Tool Required To Fix`))
    (return)))

(fn `UserConstructionScript`
  (bind _hazardeffect (`self.HazardEffect`))
  ;[1 1 1] This defines the positioning of the hazard
  (set `self.Hazard Base Nature` (`self.Nature of Hazard`))
  (switch `/Game/Blueprints/HazardAssets/HazardPositioning` (`self.Hazard Positioning`)
    (:`NewEnumerator0`
      (`SceneComponent.K2_SetRelativeLocationAndRotation` :`self` (`self.HazardEffectApplyRange`) :`NewLocation` (0.0 0.0 30.0)))
    (:`NewEnumerator1`
      (`SceneComponent.K2_SetRelativeLocationAndRotation` (`self.HazardEffectApplyRange`) (30.0 0.0 0.0) (struct :`Pitch` 90.0) false false))
    (:`NewEnumerator2`
      (`SceneComponent.K2_SetRelativeLocationAndRotation` (`self.HazardEffectApplyRange`) (`self.Hazard Location`) (`KismetMathLibrary.MakeRotator` 0.0 (`self.Hazard Rotation`)) false false)))
  (switch `/Game/Blueprints/HazardAssets/NatureOfHazard` (`self.Nature of Hazard`)
    (:`NewEnumerator4`
      (`ParticleSystemComponent.SetTemplate` (`self.HazardEffect`) "/Game/StarterContent/Particles/P_Steam_Lit.P_Steam_Lit"))
    (:`NewEnumerator0`
      (`ParticleSystemComponent.SetTemplate` _hazardeffect "/Game/ArtFolder/Particles/M5VFXVOL2/Particles/Fire/Fire_03.Fire_03")
      (`SceneComponent.SetWorldScale3D` _hazardeffect (2.0 1.0 2.0)))
    (:`NewEnumerator3`
      (`ParticleSystemComponent.SetTemplate` (`self.HazardEffect`) "/Game/StarterContent/Particles/P_Sparks.P_Sparks"))
    (:`NewEnumerator7`
      (`ParticleSystemComponent.SetTemplate` (`self.HazardEffect`) "/Game/StarterContent/Particles/P_Fire.P_Fire")
      (`StaticMeshComponent.SetStaticMesh` (`self.Hazard Unique Mesh`) "/Game/ArtFolder/Art/Meshes/Environment/Pipes/Pipe_ShortL.Pipe_ShortL")
      (`PrimitiveComponent.SetCollisionObjectType` (`self.Fix Range`) "ECC_GameTraceChannel2"))))