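; BP_NutrientPaste is a hazard actor that temporarily changes the walk speed of a character overlapping it.
; On overlap it casts to BaseCharacter, multiplies MaxWalkSpeed by a configurable amount, then restores the saved value after a configurable delay.
; A DoOnce that is never reset precedes the cast, so only the first overlapping actor of any type can trigger it.
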(event `self.ReceiveActorBeginOverlap`
  (params (OtherActor :type "Actor Object Reference"))
  (`/Engine/EditorBlueprintResources/StandardMacros.DoOnce` false
    (:`Completed`
      (bind _asbase_character (cast `/Game/Blueprints/CharacterStuff/BaseCharacter` OtherActor))
      (`/Engine/EditorBlueprintResources/StandardMacros.IsValid` _asbase_character
        (:`Is Valid`
          (bind _charactermovement (`Character.CharacterMovement` _asbase_character))
          (bind _maxwalkspeed (`CharacterMovementComponent.MaxWalkSpeed` _charactermovement))
          (set `self.TempWalkSpeed` _maxwalkspeed)
          (set `CharacterMovementComponent.MaxWalkSpeed` (* _maxwalkspeed (`self.NutrientPaste_SpeedChange_Amount`)) _charactermovement)
          (`KismetSystemLibrary.Delay` (`self.NutrientPaste_SpeedChange_Duration`))
          (set `CharacterMovementComponent.MaxWalkSpeed` (`self.TempWalkSpeed`) _charactermovement))))))

(fn `UserConstructionScript`)