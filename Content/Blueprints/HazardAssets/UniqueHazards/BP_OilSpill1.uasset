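; BP_OilSpill1 is an oil spill hazard that makes an overlapping BaseCharacter slip for a set duration.
; On overlap it scales walk speed, overrides ground friction and sets the character's OilSlicked flag.
; After a delay it restores hard-coded speed and friction values, leaving the saved TempWalkSpeed unused.
; One OilSlipTrue flag per spill blocks retriggering by any actor meanwhile, with debug prints reporting each state.
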(event `self.ReceiveActorBeginOverlap`
  (params (OtherActor :type "Actor Object Reference"))
  (if (`self.OilSlipTrue?`)
    (`KismetSystemLibrary.PrintString` "Already Oil Slip!")
    (else
      (bind _asbase_character (cast `/Game/Blueprints/CharacterStuff/BaseCharacter` OtherActor))
      (`/Engine/EditorBlueprintResources/StandardMacros.IsValid` _asbase_character
        (:`Is Valid`
          (set `self.OilSlipTrue?` true)
          (bind _charactermovement (`Character.CharacterMovement` _asbase_character))
          (bind _maxwalkspeed (`CharacterMovementComponent.MaxWalkSpeed` _charactermovement))
          (set `self.TempWalkSpeed` _maxwalkspeed)
          (set `CharacterMovementComponent.MaxWalkSpeed` (* _maxwalkspeed (`self.OilSpill_SpeedChange_Amount`)) _charactermovement)
          (set `/Game/Blueprints/CharacterStuff/BaseCharacter.OilSlicked` true _asbase_character)
          (set `CharacterMovementComponent.GroundFriction` (`self.OilFriction`) _charactermovement)
          (`KismetSystemLibrary.PrintString` "Oil Slip!")
          (`KismetSystemLibrary.Delay` (`self.OilSpill_SpeedChange_Duration`))
          (set `CharacterMovementComponent.MaxWalkSpeed` 450.0 _charactermovement)
          (set `/Game/Blueprints/CharacterStuff/BaseCharacter.OilSlicked` false _asbase_character)
          (set `CharacterMovementComponent.GroundFriction` 8.0 _charactermovement)
          (set `self.OilSlipTrue?` false)
          (`KismetSystemLibrary.PrintString` "Regular Speed"))))))

(fn `UserConstructionScript`)