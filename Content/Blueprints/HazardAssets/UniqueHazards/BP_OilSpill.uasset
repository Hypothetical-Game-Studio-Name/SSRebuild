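; BP_OilSpill is a hazard actor that temporarily alters the walk speed of a BaseCharacter that overlaps it.
; Overlap scales MaxWalkSpeed by OilSpillSpeedChangeAmount and sets OilSlicked, then restores the saved speed and clears the flag after OilSpillSpeedChangeDuration.
; A DoOnce shared across all overlapping actors gates the effect and resets on any end overlap, while the timed restore runs independently of leaving the spill.
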(event `self.ReceiveActorBeginOverlap`
  (params (OtherActor :type "Actor Object Reference"))
  (`/Engine/EditorBlueprintResources/StandardMacros.DoOnce` false :!label _label
    (:`Completed`
      (bind _asbase_character (cast `/Game/Blueprints/CharacterStuff/BaseCharacter` OtherActor))
      (`/Engine/EditorBlueprintResources/StandardMacros.IsValid` _asbase_character
        (:`Is Valid`
          (bind _charactermovement (`Character.CharacterMovement` _asbase_character))
          (bind _maxwalkspeed (`CharacterMovementComponent.MaxWalkSpeed` _charactermovement))
          (set `self.TempWalkSpeed` _maxwalkspeed)
          (set `CharacterMovementComponent.MaxWalkSpeed` (* _maxwalkspeed (`self.OilSpill_SpeedChange_Amount`)) _charactermovement)
          (set `/Game/Blueprints/CharacterStuff/BaseCharacter.OilSlicked` true _asbase_character)
          (`KismetSystemLibrary.Delay` (`self.OilSpill_SpeedChange_Duration`))
          (set `CharacterMovementComponent.MaxWalkSpeed` (`self.TempWalkSpeed`) _charactermovement)
          (set `/Game/Blueprints/CharacterStuff/BaseCharacter.OilSlicked` false _asbase_character))))))

(event `self.ReceiveActorEndOverlap`
  (params (OtherActor :type "Actor Object Reference"))
  (goto _label :!via `Reset`))

(fn `UserConstructionScript`)