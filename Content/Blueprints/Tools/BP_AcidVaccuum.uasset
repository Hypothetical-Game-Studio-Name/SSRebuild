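; BP_AcidVaccuum is an acid vacuum tool that stores collected acid units in limited-capacity tanks.
; It extends a parent tool, passing use through to the parent only while the tanks are not full.
; Each fill event increments the stored acid, prints a debug message, and flags the tanks full at capacity, clamping any overflow.
; Passover functions save and restore charge and acid levels through a ToolInformation struct.
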(event `self.ToolIsUsed`
  (params (HazardToEffect :type "/Game/Blueprints/HazardAssets/CoreHazardClass Object Reference"))
  (if (not (`self.Are Acid Tanks full?`))
    (`parent.ToolIsUsed` null)))

(event `Fill Acid Tanks`
  (bind _result (`/Engine/EditorBlueprintResources/StandardMacros.IncrementInt` (`self.Acid Contained`))
    (:`  `
      (`KismetSystemLibrary.PrintString` (`KismetStringLibrary.Concat_StrStr` "There is:" (`KismetStringLibrary.Conv_IntToString` _result) " Acidic Units in tanks") true true (struct :`G` 1.0 :`B` 0.008756 :`A` 1.0) 5.0)
      (`/Engine/EditorBlueprintResources/StandardMacros.CompareInt` _result (`self.Max Containable Acid`)
        (:`>`
          (set `self.Are Acid Tanks full?` true)
          (set `self.Acid Contained` (`self.Max Containable Acid`)))
        (:`==`
          (set `self.Are Acid Tanks full?` true))))))

(fn `Set tool passover Information`
  (set `self.Tool Information To Pass Over` (make `/Game/Blueprints/Tools/ToolInformation` (`self.Charge`) (`self.Max Charge`) (`self.Acid Contained`) (`self.Max Containable Acid`)))
  (return))

(fn `Set Tool Variables from passover`
  (params (`Tool Info to set` :type "/Game/Blueprints/Tools/ToolInformation Structure"))
  (bind (_toolcharge _maxtoolcharge _acidintanks _maxacidintanks) (break `/Game/Blueprints/Tools/ToolInformation` `Tool Info to set`))
  (set `self.Charge` _toolcharge)
  (set `self.Max Charge` _maxtoolcharge)
  (set `self.Acid Contained` _acidintanks)
  (set `self.Max Containable Acid` _maxacidintanks)
  (return))

(fn `UserConstructionScript`
  (`parent.UserConstructionScript`))