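; AnthonyFunctionLibrary is a Blueprint tool asset whose one function, Characterbuttonactivation, has an empty body and does nothing when called.
; Its disconnected nodes sketch a short visibility trace from CastArrowTarget that activates a hit BP_SimpleButton.
; They also sketch picking up overlapping BP_BaseTool actors by swapping EquippedTool's child actor class and setting CurrentTool, a step commented as not working.
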(fn `Characterbuttonactivation`)