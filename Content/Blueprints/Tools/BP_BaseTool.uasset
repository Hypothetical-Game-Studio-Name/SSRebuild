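; Base actor for player-held tools that can be used continuously, thrown and picked up again.
; Use runs a looping timer that spawns projectiles from the player's cast arrow with sound and particles, draining charge on battery tools until empty.
; It gets the player through its parent actor and flags hammer state on them.
; Throwing enables physics and applies an impulse, while an information struct carries charge between tool instances.
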(event `self.ReceiveBeginPlay`
  ;[1 1 1] When the tool is created, this will check if the player character is using a hammer.
  (`KismetSystemLibrary.Delay` 0.1)
  (`self.Check if hammer tool is being used by player`))

(event `ToolStoppedBeingUsed`
  (bind _firingsound (`self.FiringSound`))
  ;[1 1 1] When the player presses the use tool input, this bp fires
  (`KismetSystemLibrary.K2_ClearAndInvalidateTimerHandle` (stale `ToolIsUsed` _returnvalue))
  (set `/Game/Blueprints/CharacterStuff/BaseCharacter.Is hammer tool being used?` false (`self.Player Character Refrence`))
  (`AudioComponent.Stop` _firingsound)
  (`ActorComponent.Deactivate` _firingsound)
  (`ActorComponent.Deactivate` (`self.Tool Particle Effect`))
  (`self.Unlock Particle DoOnce`))

(event `ToolIsUsed`
  (params (HazardToEffect :type "/Game/Blueprints/HazardAssets/CoreHazardClass Object Reference"))
  ;[1 1 1] When the player presses the use tool input, this bp fires
  (`ActorComponent.Activate` (`self.FiringSound`) false)
  (`|ExecutionSequence`
    (:`then_0`
      (if (`self.BatteryBasedTool`) :!label _label
        (if (> (`self.Charge`) 0)
          (`self.PlaySound`)
          (`self.Check Particle Need Activating`)
          (bind _result (`/Engine/EditorBlueprintResources/StandardMacros.DecrementInt` (`self.Charge`))
            (:`  `
              (`self.Update Tool Charge` _result)
              (`|SpawnActorFromClass` (`self.What Projectile?`) (`SceneComponent.K2_GetComponentToWorld` (`/Game/Blueprints/CharacterStuff/BaseCharacter.Cast Arrow Target` (`self.Player Character Refrence`))) "Undefined" "OverrideRootScale" self null :!label _label_2)))
          (else
            (`GameplayStatics.PlaySoundAtLocation` "/Game/Sounds/SoundCues/SC_Error.SC_Error" (`self.K2_GetActorLocation`) (struct) 1.0 1.0 0.0 null null null)
            (`self.ToolStoppedBeingUsed`)))
        (else
          (set `/Game/Blueprints/CharacterStuff/BaseCharacter.Is hammer tool being used?` true (`self.Player Character Refrence`))
          (`self.Check Particle Need Activating`)
          (`self.PlaySound`)
          (goto _label_2))))
    (:`then_1`
      (bind _returnvalue (`KismetSystemLibrary.K2_SetTimerDelegate` (delegate `Tool Fire`) 0.1 true)))))

(event `Tool Fire`
  ;[1 1 1] When the player presses the use tool input, this bp fires
  (goto _label))

(event `Check Particle Need Activating`
  ;[1 1 1] When the player presses the use tool input, this bp fires
  (`/Engine/EditorBlueprintResources/StandardMacros.DoOnce` false :!label _label_3
    (:`Completed`
      (`self.Activate Tool Effect`))))

(event `PlaySound`
  ;[1 1 1] When the player presses the use tool input, this bp fires
  (`self.Commence Firing Sound`))

(event `Unlock Particle DoOnce`
  ;[1 1 1] When the player presses the use tool input, this bp fires
  (goto _label_3 :!via `Reset`))

(event `Activate Tool Effect`
  ;[1 1 1] When the player presses the use tool input, this bp fires
  (`ActorComponent.Activate` (`self.Tool Particle Effect`) true))

(event `Tool is thrown`
  (params (`Throw / Drop Strength` :type "Float (double-precision)"))
  ;[1 1 1] These are the instructions for how a tool is thrown.
  (set `self.Throw Drop Strength` `Throw / Drop Strength`)
  (`SceneComponent.SetHiddenInGame` (`self.Arrow`) true false)
  (`self.Set collision for physics once thrown`)
  (`|ExecutionSequence`
    (:`then_0`
      (`PrimitiveComponent.SetSimulatePhysics` (`self.ToolMesh`) true))
    (:`then_1`
      (`PrimitiveComponent.AddImpulse` (`self.ToolMesh`) (`self.Get throw direction and strength`) "None" true))))

(fn `Check if hammer tool is being used by player`
  (bind _player_character_refrence (message `/Game/Blueprints/Interfaces/PlayerCharacterInterface/SolarSailorPlayerCharacterRefrenceGetter.Player Character Refrence Getter` (`self.GetParentActor`)))
  (`/Engine/EditorBlueprintResources/StandardMacros.IsValid` _player_character_refrence
    (:`Is Valid`
      (set `self.Player Character Refrence` _player_character_refrence)
      (set `/Game/Blueprints/CharacterStuff/BaseCharacter.Is hammer tool being held?` (`|EnumEquality` (`self.What tool is this?`) "NewEnumerator0") _player_character_refrence))))

(fn `Commence Firing Sound`
  (if (`AudioComponent.IsPlaying` (`self.FiringSound`))
    (return)
    (else
      (`AudioComponent.Play` (`self.FiringSound`) 0.0)
      (return))))

(fn `F_ExpendBatteryLife`
  (params (Seconds :type "Float (double-precision)")))

(fn `F_ToolEffect`
  (params (HazardToEffect :type "/Game/Blueprints/HazardAssets/CoreHazardClass Object Reference"))
  (message `/Game/Blueprints/Interfaces/PlayerCharacterInterface/SolarSailorPlayerCharacterRefrenceGetter.Player Character Refrence Getter` (`self.GetParentActor`)))

(fn `Get throw direction and strength`
  (returns (ReturnValue :type "Vector Structure"))
  (return (* (`KismetMathLibrary.GetForwardVector` (`SceneComponent.K2_GetComponentRotation` (`self.Tool Sphere`))) (`self.Throw Drop Strength`))))

(fn `Get tool Info`
  (returns (`Tool Ref` :type "/Game/Blueprints/Tools/BP_BaseTool Object Reference"))
  (return self))

(fn `Set collision for physics once thrown`
  (bind _toolmesh (`self.ToolMesh`))
  (`PrimitiveComponent.SetCollisionResponseToAllChannels` _toolmesh "ECR_Block")
  (`PrimitiveComponent.SetCollisionResponseToChannel` _toolmesh "ECC_Pawn" "ECR_Ignore")
  (`PrimitiveComponent.SetCollisionResponseToChannel` _toolmesh "ECC_WorldDynamic" "ECR_Overlap")
  (`PrimitiveComponent.SetCollisionEnabled` _toolmesh "QueryAndPhysics")
  (`PrimitiveComponent.SetCollisionObjectType` _toolmesh "ECC_PhysicsBody")
  (set `self.Can Be picked up?` true)
  (set `PrimitiveComponent.bGenerateOverlapEvents` true _toolmesh)
  (return))

(fn `Set tool passover Information`
  (set `self.Tool Information To Pass Over` (make `/Game/Blueprints/Tools/ToolInformation` (`self.Charge`) (`self.Max Charge`)))
  (return))

(fn `Set Tool Variables from passover`
  (params (`Tool Info to set` :type "/Game/Blueprints/Tools/ToolInformation Structure"))
  (bind (_toolcharge _maxtoolcharge) (break `/Game/Blueprints/Tools/ToolInformation` `Tool Info to set`))
  (set `self.Charge` _toolcharge)
  (set `self.Max Charge` _maxtoolcharge)
  (return))

(fn `Update Tool Charge`
  (params (InputPin :type Integer))
  (set `self.Tool Information To Pass Over` (make `/Game/Blueprints/Tools/ToolInformation` InputPin (`self.Max Charge`)))
  (return))

(fn `UserConstructionScript`)