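; BP_ElectricGun is a tool Blueprint that roots the player in place while it is in use.
; On use, it gets the player character through an interface message on its parent actor, then stops and deactivates the character's movement component.
; When use stops, it reactivates movement with a reset, and both events then call the parent class's implementation.
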(event `self.ToolStoppedBeingUsed`
  (bind _player_character_refrence (message `/Game/Blueprints/Interfaces/PlayerCharacterInterface/SolarSailorPlayerCharacterRefrenceGetter.Player Character Refrence Getter` (`self.GetParentActor`)))
  (`ActorComponent.Activate` (`Character.CharacterMovement` _player_character_refrence) true)
  (`parent.ToolStoppedBeingUsed`))

(event `self.ToolIsUsed`
  (params (HazardToEffect :type "/Game/Blueprints/HazardAssets/CoreHazardClass Object Reference"))
  (bind _player_character_refrence (message `/Game/Blueprints/Interfaces/PlayerCharacterInterface/SolarSailorPlayerCharacterRefrenceGetter.Player Character Refrence Getter` (`self.GetParentActor`)))
  (bind _charactermovement (`Character.CharacterMovement` _player_character_refrence))
  (`NavMovementComponent.StopActiveMovement` _charactermovement)
  (`ActorComponent.Deactivate` _charactermovement)
  (`parent.ToolIsUsed` null))

(fn `UserConstructionScript`
  (`parent.UserConstructionScript`))