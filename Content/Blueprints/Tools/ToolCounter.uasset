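; Interactable counter actor that displays a tool on a bobbing, spinning child actor and lets characters take, store or swap tools.
; Interaction branches on the character's tool type and whether one is stored, giving back a hammer when a tool is deposited.
; Exchanges swap child actor classes, copying each tool's state through passover data.
; An outline is added as a duplicate mesh with an outline material.
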(event `self.ReceiveBeginPlay`
  (`/Engine/EditorBlueprintResources/StandardMacros.IsValid` (`ChildActorComponent.ChildActor` (`self.Tooltohold`))
    (:`Is Valid`
      (set `self.Tool Stored?` true)
      (`|ExecutionSequence`
        (:`then_0`
          (bind (_direction _tool_bob) (`Timeline|Tool movement` :!label _label)
            (:`Update`
              (`SceneComponent.K2_SetRelativeLocation` (`self.Tooltohold`) _tool_bob false false)
              (`SceneComponent.K2_AddRelativeRotation` (`self.Tooltohold`) (`KismetMathLibrary.MakeRotator` 0.0 0.0 0.5) false false))))
        (:`then_1`
          (`self.Outline Tool` :!label _label_2))))
    (:`Is Not Valid`
      (set `self.Tool Stored?` false)
      (goto _label))))

(event `/Game/Blueprints/Interfaces/InteractEvent.Is interacted with`
  (params (`Character who interacts` :type "/Game/Blueprints/CharacterStuff/BaseCharacter Object Reference"))
  (`self.Exchange or store tool` `Character who interacts`)
  (goto _label_2))

(fn `Exchange or store tool`
  (params (`Character Input` :type "/Game/Blueprints/CharacterStuff/BaseCharacter Object Reference"))
  (locals (`Character Refrence` :type "/Game/Blueprints/CharacterStuff/BaseCharacter Object Reference") (`Hold Character Current Tool Class` :type "Actor Class Reference") (`Hold Character Tool Info` :type "/Game/Blueprints/Tools/ToolInformation Structure"))
  (bind _output_get (set `local.Character Refrence` `Character Input`))
  (bind _tool_ref (message `/Game/Blueprints/Interfaces/ToolInterafce.Get tool Info` (`ChildActorComponent.ChildActor` (`/Game/Blueprints/CharacterStuff/BaseCharacter.EquippedTool` _output_get))))
  (if (`|EnumEquality` (`/Game/Blueprints/Tools/BP_BaseTool.What tool is this?` _tool_ref) "NewEnumerator0")
    (if (`self.Tool Stored?`)
      (bind _tool_ref_2 (message `/Game/Blueprints/Interfaces/ToolInterafce.Get tool Info` (`ChildActorComponent.ChildActor` (`self.Tooltohold`))))
      (`/Game/Blueprints/Tools/BP_BaseTool.Set tool passover Information` _tool_ref_2)
      (`ChildActorComponent.SetChildActorClass` (`/Game/Blueprints/CharacterStuff/BaseCharacter.EquippedTool` (`local.Character Refrence`)) (`GameplayStatics.GetObjectClass` _tool_ref_2))
      (bind _tool_ref_3 (message `/Game/Blueprints/Interfaces/ToolInterafce.Get tool Info` (`ChildActorComponent.ChildActor` (`/Game/Blueprints/CharacterStuff/BaseCharacter.EquippedTool` (`local.Character Refrence`)))))
      (`/Game/Blueprints/Tools/BP_BaseTool.Set Tool Variables from passover` _tool_ref_3 (`/Game/Blueprints/Tools/BP_BaseTool.Tool Information To Pass Over` _tool_ref_2))
      (`ChildActorComponent.SetChildActorClass` (`self.Tooltohold`) null)
      (set `self.Tool Stored?` false)
      (return))
    (elif (`self.Tool Stored?`)
      (bind _tool_ref_4 (message `/Game/Blueprints/Interfaces/ToolInterafce.Get tool Info` (`ChildActorComponent.ChildActor` (`/Game/Blueprints/CharacterStuff/BaseCharacter.EquippedTool` (`local.Character Refrence`)))))
      (`/Game/Blueprints/Tools/BP_BaseTool.Set tool passover Information` _tool_ref_4)
      (set `local.Hold Character Tool Info` (`/Game/Blueprints/Tools/BP_BaseTool.Tool Information To Pass Over` _tool_ref_4))
      (set `local.Hold Character Current Tool Class` (`GameplayStatics.GetObjectClass` _tool_ref_4))
      (bind _tool_ref_5 (message `/Game/Blueprints/Interfaces/ToolInterafce.Get tool Info` (`ChildActorComponent.ChildActor` (`self.Tooltohold`))))
      (`/Game/Blueprints/Tools/BP_BaseTool.Set tool passover Information` _tool_ref_5)
      (`ChildActorComponent.SetChildActorClass` (`/Game/Blueprints/CharacterStuff/BaseCharacter.EquippedTool` (`local.Character Refrence`)) (`GameplayStatics.GetObjectClass` _tool_ref_5))
      (bind _tool_ref_6 (message `/Game/Blueprints/Interfaces/ToolInterafce.Get tool Info` (`ChildActorComponent.ChildActor` (`/Game/Blueprints/CharacterStuff/BaseCharacter.EquippedTool` (`local.Character Refrence`)))))
      (`/Game/Blueprints/Tools/BP_BaseTool.Set Tool Variables from passover` _tool_ref_6 (`/Game/Blueprints/Tools/BP_BaseTool.Tool Information To Pass Over` _tool_ref_5))
      (`ChildActorComponent.SetChildActorClass` (`self.Tooltohold`) (`local.Hold Character Current Tool Class`))
      (bind _tool_ref_7 (message `/Game/Blueprints/Interfaces/ToolInterafce.Get tool Info` (`ChildActorComponent.ChildActor` (`self.Tooltohold`))))
      (`/Game/Blueprints/Tools/BP_BaseTool.Set Tool Variables from passover` _tool_ref_7 (`local.Hold Character Tool Info`))
      (set `self.Tool Stored?` true)
      (return)
      (else
        (bind _tool_ref_8 (message `/Game/Blueprints/Interfaces/ToolInterafce.Get tool Info` (`ChildActorComponent.ChildActor` (`/Game/Blueprints/CharacterStuff/BaseCharacter.EquippedTool` (`local.Character Refrence`)))))
        (`/Game/Blueprints/Tools/BP_BaseTool.Set tool passover Information` _tool_ref_8)
        (`ChildActorComponent.SetChildActorClass` (`self.Tooltohold`) (`GameplayStatics.GetObjectClass` _tool_ref_8))
        (bind _tool_ref_9 (message `/Game/Blueprints/Interfaces/ToolInterafce.Get tool Info` (`ChildActorComponent.ChildActor` (`self.Tooltohold`))))
        (`/Game/Blueprints/Tools/BP_BaseTool.Set Tool Variables from passover` _tool_ref_9 (`/Game/Blueprints/Tools/BP_BaseTool.Tool Information To Pass Over` _tool_ref_8))
        (`ChildActorComponent.SetChildActorClass` (`/Game/Blueprints/CharacterStuff/BaseCharacter.EquippedTool` (`local.Character Refrence`)) "/Game/Blueprints/Tools/BP_HammerTool.BP_HammerTool_C")
        (set `self.Tool Stored?` true)
        (return)))))

(fn `Get and store player tool`
  (params (`Actor Ref` :type "Actor Object Reference"))
  ;[1 1 1] This talks to the player pawn, and removes their currently selected tool, setting the 'Tooltohold' child actor to that tool
  (set `self.Tool This counter holds` null))

(fn `Outline Tool`
  (bind _childactor (`ChildActorComponent.ChildActor` (`self.Tooltohold`)))
  (`/Engine/EditorBlueprintResources/StandardMacros.IsValid` _childactor
    (:`Is Valid`
      (bind _tool_ref (message `/Game/Blueprints/Interfaces/ToolInterafce.Get tool Info` _childactor))
      (bind _returnvalue (`AddComponent|NODE_AddStaticMeshComponent-0` :`self` _tool_ref :`bManualAttachment` true))
      (`PrimitiveComponent.SetCollisionEnabled` _returnvalue "NoCollision")
      (bind _toolmesh (`/Game/Blueprints/Tools/BP_BaseTool.ToolMesh` _tool_ref))
      (`StaticMeshComponent.SetStaticMesh` _returnvalue (`StaticMeshComponent.StaticMesh` _toolmesh))
      (`SceneComponent.K2_AttachToComponent` _returnvalue _toolmesh "None" "SnapToTarget" "SnapToTarget" "SnapToTarget" true)
      (`PrimitiveComponent.SetMaterial` _returnvalue 0 "/Game/Blueprints/Tools/Outline_Inst.Outline_Inst")
      (return))))

(fn `UserConstructionScript`
  (`ChildActorComponent.SetChildActorClass` (`self.Tooltohold`) (`self.Tool This counter holds`)))