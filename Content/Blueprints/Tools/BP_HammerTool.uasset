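; BP_HammerTool is a tool Blueprint that repairs breach hazards.
; Its F_ToolEffect function validates the hazard passed in, switches on its nature and, for a Breach, calls that hazard's small breach repair event.
; The event graph holds only disabled default events, and the construction script just calls its parent, so all of the tool's own behavior lives in that function.
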(fn `F_ToolEffect`
  (params (HazardToEffect :type "/Game/Blueprints/HazardAssets/CoreHazardClass Object Reference"))
  (`/Engine/EditorBlueprintResources/StandardMacros.IsValid` HazardToEffect
    (:`Is Valid`
      (switch `/Game/Blueprints/HazardAssets/NatureOfHazard` (`/Game/Blueprints/HazardAssets/CoreHazardClass.Nature of Hazard` HazardToEffect)
        (:`NewEnumerator4`
          (`/Game/Blueprints/HazardAssets/CoreHazardClass.Small Breach Repair Event` HazardToEffect))))))

(fn `UserConstructionScript`
  (`parent.UserConstructionScript`))