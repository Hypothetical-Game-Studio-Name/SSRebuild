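; WillWindow is a blockout window that loses health when hit by a hammer repair orb.
; Overlaps on the FixRange collision cast to ToolProjectileMaster, then HammerRepairOrb, and each match removes one point of WindowHealth.
; At zero or below, it destroys the BreakableMesh and FixRange components, leaving the actor in place, and spawns a scaled-down firework burst at EmitterLocation.
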(event `self.Fix Range.OnComponentBeginOverlap`
  (params (OverlappedComponent :type "PrimitiveComponent Object Reference") (OtherActor :type "Actor Object Reference") (OtherComp :type "PrimitiveComponent Object Reference") (OtherBodyIndex :type Integer) (bFromSweep :type Boolean) (SweepResult :type "HitResult Structure (by ref)"))
  ;[1 1 1] Hammer Repair Orb overlap with Window Collision
  (bind _astool_projectile_master (cast `/Game/Blueprints/Tools/Projectiles/ToolProjectileMaster` OtherActor))
  (bind _ashammer_repair_orb (cast `/Game/Blueprints/Tools/Projectiles/HammerRepairOrb` _astool_projectile_master))
  ;[1 1 1] Remove Health
  (set `self.WindowHealth` (- (`self.WindowHealth`) 1))
  ;[1 1 1] Is Health <= 0?
  (if (<= (`self.WindowHealth`) 0)
    ;[1 1 1] Destroy Window and Collision
    (`ActorComponent.K2_DestroyComponent` (`self.BreakableMesh`))
    (`ActorComponent.K2_DestroyComponent` (`self.Fix Range`))
    (`GameplayStatics.SpawnEmitterAtLocation` "/Game/ArtFolder/Particles/TS_Fireworks/Particles/PS_TS_Fireworks_Burst_ShellsWithinShells.PS_TS_Fireworks_Burst_ShellsWithinShells" (`SceneComponent.K2_GetComponentLocation` (`self.EmitterLocation`)) (struct) (0.05 0.05 0.05))))

(fn `UserConstructionScript`)