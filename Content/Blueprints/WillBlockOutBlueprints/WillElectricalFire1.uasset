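; Electrical fire hazard that cycles on and off, killing the player on contact until a tool projectile disables it.
; Timers and delays run the loop: warning lights turn red, ShootFlame shows the fire and sweeps the kill box into place, then DisableEvent reverses this and turns them green.
; Any ToolProjectileMaster entering FixRange destroys the fire components and pauses the ShootFlame timer, though the Charge Tool is intended.
; Tick spins the light mesh.
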(event `self.ReceiveBeginPlay`
  ;[1 1 1] Set Kill Collision off and Initialise Flame
  (`PrimitiveComponent.SetCollisionEnabled` (`self.PlayerKillBox`) "NoCollision")
  (`self.InitialiseFlame`))

(event `self.PlayerKillBox.OnComponentBeginOverlap`
  (params (OverlappedComponent :type "PrimitiveComponent Object Reference") (OtherActor :type "Actor Object Reference") (OtherComp :type "PrimitiveComponent Object Reference") (OtherBodyIndex :type Integer) (bFromSweep :type Boolean) (SweepResult :type "HitResult Structure (by ref)"))
  ;[1 1 1] Set Kill Box to kill Player
  (`KismetSystemLibrary.PrintString` "Before Branch")
  (if (`self.FireSpawning?`)
    (bind _asbase_character (cast `/Game/Blueprints/CharacterStuff/BaseCharacter` OtherActor)
      (:`then`
        (`/Game/Blueprints/CharacterStuff/BaseCharacter.Hazard Death Event` _asbase_character "NewEnumerator0"))
      (:`CastFailed`
        (`KismetSystemLibrary.PrintString` "Player Collision - Cast Failed")))
    (else
      (`KismetSystemLibrary.PrintString` "FireSpawnFalse"))))

(event `StopFlame`
  ;[1 1 1] Stop the Flame (Pause)
  (`KismetSystemLibrary.K2_SetTimerDelegate` (delegate `DisableEvent`) 10.0))

(event `DisableEvent`
  (bind _playerkillbox (`self.PlayerKillBox`))
  ;[1 1 1] Disable Flame
  (`SceneComponent.SetVisibility` (`self.PointLightFire`) false false)
  (`SceneComponent.ToggleVisibility` (`self.ParticleSystemFire`) false)
  (`PrimitiveComponent.SetCollisionEnabled` _playerkillbox "NoCollision")
  (set `self.FireSpawning?` false)
  (`SceneComponent.K2_SetWorldLocation` _playerkillbox (`SceneComponent.K2_GetComponentLocation` (`self.KillBoxMoveLocation`)) true false)
  (`LightComponent.SetLightColor` (`self.WarningLight`) (struct :`R` 0.004777 :`G` 1.0 :`A` 1.0) true)
  (`LightComponent.SetLightColor` (`self.WarningLight1`) (struct :`R` 0.004777 :`G` 1.0 :`A` 1.0) true)
  (`KismetSystemLibrary.Delay` 8.0)
  (`self.InitialiseFlame`))

(event `InitialiseFlame`
  ;[1 1 1] Set Countown to Flame and change light colour
  (`LightComponent.SetLightColor` (`self.WarningLight`) (struct :`R` 1.0 :`B` 0.06219 :`A` 1.0) true)
  (`LightComponent.SetLightColor` (`self.WarningLight1`) (struct :`R` 1.0 :`B` 0.06219 :`A` 1.0) true)
  (`KismetSystemLibrary.Delay` 4.0)
  (`KismetSystemLibrary.K2_SetTimer` null "ShootFlame" 1.0))

(event `self.Fix Range.OnComponentBeginOverlap`
  (params (OverlappedComponent :type "PrimitiveComponent Object Reference") (OtherActor :type "Actor Object Reference") (OtherComp :type "PrimitiveComponent Object Reference") (OtherBodyIndex :type Integer) (bFromSweep :type Boolean) (SweepResult :type "HitResult Structure (by ref)"))
  ;[1 1 1] Deactivate Electrical Fire with Charge Tool (Currently works with any Tool)
  (cast `/Game/Blueprints/Tools/Projectiles/ToolProjectileMaster` OtherActor)
  (`self.DeactivateFlame`))

(event `DeactivateFlame`
  ;[1 1 1] Permanently disactivate Flame and set light colour to Green
  (`ActorComponent.K2_DestroyComponent` (`self.Fix Range`))
  (`ActorComponent.K2_DestroyComponent` (`self.PointLightFire`))
  (`ActorComponent.K2_DestroyComponent` (`self.ParticleSystemFire`))
  (`ActorComponent.K2_DestroyComponent` (`self.PlayerKillBox`))
  (`ActorComponent.K2_DestroyComponent` (`self.ParticleChargeToolInteract`))
  (`KismetSystemLibrary.K2_PauseTimer` null "ShootFlame")
  (`LightComponent.SetLightColor` (`self.WarningLight`) (struct :`R` 0.004777 :`G` 1.0 :`A` 1.0) true)
  (`LightComponent.SetLightColor` (`self.WarningLight1`) (struct :`R` 0.004777 :`G` 1.0 :`A` 1.0) true))

(event `self.ReceiveTick`
  (params (DeltaSeconds :type "Float (single-precision)"))
  ;[1 1 1] Rotate the Lights on Tick
  (`SceneComponent.K2_AddLocalRotation` (`self.SpinningMesh`) (`KismetMathLibrary.MakeRotator` 0.0 0.0 (* DeltaSeconds (`self.Rotation`))) false false))

(fn `ShootFlame`
  (bind _playerkillbox (`self.PlayerKillBox`))
  (`SceneComponent.ToggleVisibility` (`self.ParticleSystemFire`) false)
  (`SceneComponent.SetVisibility` (`self.PointLightFire`) true false)
  (`PrimitiveComponent.SetCollisionEnabled` _playerkillbox "QueryAndPhysics")
  (`SceneComponent.K2_SetWorldLocation` _playerkillbox (`SceneComponent.K2_GetComponentLocation` (`self.KillBoxKillLocation`)) true false)
  (set `self.FireSpawning?` true)
  (`self.StopFlame`))

(fn `UserConstructionScript`)