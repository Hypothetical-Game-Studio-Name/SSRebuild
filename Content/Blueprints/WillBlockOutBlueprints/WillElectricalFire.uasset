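; Electrical fire hazard that cycles between a red warning, a lethal flame burst and a green safe pause, with a rotating wall lamp.
; Chained timers and delays drive the loop, toggling particles, lights, indicator icons and a kill box that triggers BaseCharacter's hazard death.
; An ElectricGunBullet entering FixRange permanently deactivates it with an explosion, hiding its effects and showing the tick icon.
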(event `self.ReceiveBeginPlay`
  ;[1 1 1] Set Kill Collision off and Initialise Flame
  (`PrimitiveComponent.SetCollisionEnabled` (`self.PlayerKillBox`) "NoCollision")
  (`self.InitialiseFlame`))

(event `self.PlayerKillBox.OnComponentBeginOverlap`
  (params (OverlappedComponent :type "PrimitiveComponent Object Reference") (OtherActor :type "Actor Object Reference") (OtherComp :type "PrimitiveComponent Object Reference") (OtherBodyIndex :type Integer) (bFromSweep :type Boolean) (SweepResult :type "HitResult Structure (by ref)"))
  ;[1 1 1] Set Kill Box to kill Player
  (if (`self.FireSpawning?`)
    (bind _asbase_character (cast `/Game/Blueprints/CharacterStuff/BaseCharacter` OtherActor))
    (`/Game/Blueprints/CharacterStuff/BaseCharacter.Hazard Death Event` _asbase_character "NewEnumerator0")))

(event `StopFlame`
  ;[1 1 1] Stop the Flame (Pause)
  (`KismetSystemLibrary.K2_SetTimerDelegate` (delegate `DisableEvent`) 2.0))

(event `DisableEvent`
  ;[1 1 1] Disable Flame
  (`SceneComponent.SetVisibility` (`self.Tick`) true false)
  (`ActorComponent.Deactivate` (`self.ParticleSystemFire`))
  (`SceneComponent.SetVisibility` (`self.Exclamation point `) false false)
  (`SceneComponent.SetVisibility` (`self.PointLightFire`) false false)
  (`PrimitiveComponent.SetCollisionEnabled` (`self.PlayerKillBox`) "NoCollision")
  (set `self.FireSpawning?` false)
  (`LightComponent.SetLightColor` (`self.WarningLight`) (struct :`R` 0.004777 :`G` 1.0 :`A` 1.0) true)
  (`LightComponent.SetLightColor` (`self.WarningLight2`) (struct :`R` 0.004777 :`G` 1.0 :`A` 1.0) true)
  (`KismetSystemLibrary.Delay` 8.0)
  (`self.InitialiseFlame`))

(event `InitialiseFlame`
  ;[1 1 1] Set Countown to Flame and change light colour
  (if (not (`self.DeactivateFlameBool`))
    (`LightComponent.SetLightColor` (`self.WarningLight`) (struct :`R` 1.0 :`B` 0.06219 :`A` 1.0) true)
    (`LightComponent.SetLightColor` (`self.WarningLight2`) (struct :`R` 1.0 :`B` 0.06219 :`A` 1.0) true)
    (`SceneComponent.SetVisibility` (`self.Tick`) false false)
    (`SceneComponent.SetVisibility` (`self.Exclamation point `) true false)
    (`KismetSystemLibrary.Delay` 2.0)
    (`ActorComponent.Activate` (`self.ParticleSystemFire`) false)
    (`KismetSystemLibrary.K2_SetTimer` null "ShootFlame" 1.0)))

(event `self.Fix Range.OnComponentBeginOverlap`
  (params (OverlappedComponent :type "PrimitiveComponent Object Reference") (OtherActor :type "Actor Object Reference") (OtherComp :type "PrimitiveComponent Object Reference") (OtherBodyIndex :type Integer) (bFromSweep :type Boolean) (SweepResult :type "HitResult Structure (by ref)"))
  ;[1 1 1] Deactivate Electrical Fire with Charge Tool
  (bind _astool_projectile_master (cast `/Game/Blueprints/Tools/Projectiles/ToolProjectileMaster` OtherActor))
  (bind _aselectric_gun_bullet (cast `/Game/Blueprints/Tools/Projectiles/ElectricGunBullet` _astool_projectile_master))
  (if (== OtherActor _aselectric_gun_bullet)
    (`self.DeactivateFlame`)))

(event `DeactivateFlame`
  ;[1 1 1] Permanently disactivate Flame/Particle Effects/Lighting/collision and permanently set tick
  (set `self.DeactivateFlameBool` true)
  (`SceneComponent.SetVisibility` (`self.PointLightFire`) false false)
  (`SceneComponent.SetVisibility` (`self.WarningLight`) false false)
  (`SceneComponent.SetVisibility` (`self.WarningLight2`) false false)
  (`SceneComponent.SetVisibility` (`self.ParticleChargeToolInteract`) false false)
  (`SceneComponent.SetVisibility` (`self.Exclamation point `) false false)
  (`SceneComponent.SetVisibility` (`self.ParticleSystemFire`) false false)
  (`SceneComponent.SetVisibility` (`self.ParticleSystemEmbers`) false false)
  (`PrimitiveComponent.SetCollisionEnabled` (`self.Fix Range`) "NoCollision")
  (`PrimitiveComponent.SetCollisionEnabled` (`self.PlayerKillBox`) "NoCollision")
  (`KismetSystemLibrary.K2_PauseTimer` null "ShootFlame")
  (`GameplayStatics.SpawnEmitterAtLocation` "/Game/StarterContent/Particles/P_Explosion.P_Explosion" (`SceneComponent.K2_GetComponentLocation` (`self.ChargeToolInteractMeshTop`)))
  (`SceneComponent.SetVisibility` (`self.Tick`) true false))

(event `self.ReceiveTick`
  (params (DeltaSeconds :type "Float (single-precision)"))
  ;[1 1 1] Rotate the Lights on Tick
  (`SceneComponent.K2_AddLocalRotation` (`self.Wall_Lamp`) (`KismetMathLibrary.MakeRotator` 0.0 0.0 (* DeltaSeconds (`self.Rotation`))) false false))

(fn `ShootFlame`
  (if (not (`self.DeactivateFlameBool`))
    (`SceneComponent.SetVisibility` (`self.PointLightFire`) true false)
    (`GameplayStatics.PlaySoundAtLocation` "/Game/Sounds/imports/FireExtinguisher/FlameThrower_Cue.FlameThrower_Cue" (`self.K2_GetActorLocation`) (struct) 1.0 1.0 0.0 null null null)
    (set `self.FireSpawning?` true)
    (`PrimitiveComponent.SetCollisionEnabled` (`self.PlayerKillBox`) "QueryAndPhysics"))
  (`self.StopFlame`))

(fn `UserConstructionScript`)